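; Game Blueprint for Neuroshima whose only implemented logic is a work-in-progress team layout check; the event graph is empty.
; NeuroCheckTeams gathers each player's team into unique and per-player lists, then branches on player and team counts toward 1v2, 1v1v1v1, 2v2 or no-team cases.
; The branches are stubs, except 2v2, which removes the first player's team from the per-player list.
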(event EventBeginPlay)

(event EventActorBeginOverlap
  (params (OtherActor :type Actor%20Object%20Reference)))

(event EventTick
  (params (DeltaSeconds :type Float%20%28single-precision%29)))

(fn ConstructionScript
  (|CallParentFunction))

(fn NeuroCheckTeams
  (bind _teams (LocalVariables|GetTeams))
  (bind _playersteams (LocalVariables|GetPlayersTeams))
  (bind _returnvalue (Utilities|Array|Length _teams))
  (for _array_element (Variables|Default|GetPlayers)
    (Utilities|Array|AddUnique (LocalVariables|GetTeams) (Variables|/Script/UnrealGames.UGPS|GetTeam _array_element))
    (Utilities|Array|Add (LocalVariables|GetPlayersTeams) (Variables|/Script/UnrealGames.UGPS|GetTeam _array_element)))
  (if (== (Utilities|Array|Length (Variables|Default|GetPlayers)) 3)
    ;[1 1 1] 1v2
    (return)
    (elif (== (Utilities|Array|Length (Variables|Default|GetPlayers)) 4)
      (if (== _returnvalue 4)
        ;[1 1 1] 1v1v1v1
        (return)
        (elif (!= _returnvalue 2)
          (return)
          (else
            (Utilities|Array|RemoveItem _playersteams (Utilities|Array|Get(acopy) _playersteams))
            ;[1 1 1] 2v2
            (return))))
      (else
        ;[1 1 1] No teams
        (return)))))