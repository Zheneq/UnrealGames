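; NeuroHand displays a hand of Neuroshima tiles on three hex slots, synced to the card group of its UGCardGroupViz.
; On each visualizer update it clears slots whose tile left the group, then assigns tiles without a board hex to the first empty slot.
; It then snaps each slotted tile to its hex's "Tile" socket, printing slot contents for debugging.
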(event UpdateVisualizer(UGCardGroupViz)
  (bind _ugcardgroupviz (Variables|Default|GetUGCardGroupViz))
  (bind _returnvalue (Class|UGCardGroupVizComponent|GetGroup _ugcardgroupviz))
  (Utilities|IsValid _returnvalue
    (:Is%20Valid
      (Utilities|FlowControl|Sequence
        (:then_0
          (CallFunction|ClearOutdated))
        (:then_1
          (for _array_element (Variables|/Script/UnrealGames.UGCardGroup|GetCards _returnvalue)
            (bind _asneuro_base_tile (Utilities|Casting|CastToNeuroBaseTile _array_element))
            (Utilities|IsValid (Variables|/Game/Games/Neuroshima/Blueprints/Tile/AbstractClasses/NeuroBaseTile.NeuroBaseTile_C|GetBoardHex _asneuro_base_tile)
              (:Is%20Not%20Valid
                (bind _array_element_2 (Utilities|Array|ForEachLoopwithBreak (Variables|Default|GetHexes) :!label _label)
                  (:LoopBody
                    (Utilities|IsValid (Variables|/Game/Games/Neuroshima/Blueprints/NeuroBoardHex.NeuroBoardHex_C|GetTile _array_element_2)
                      (:Is%20Not%20Valid
                        (Variables|/Game/Games/Neuroshima/Blueprints/NeuroBoardHex.NeuroBoardHex_C|SetTile _array_element_2 _asneuro_base_tile)
                        (Variables|/Game/Games/Neuroshima/Blueprints/Tile/AbstractClasses/NeuroBaseTile.NeuroBaseTile_C|SetBoardHex _asneuro_base_tile _array_element_2)
                        (goto _label Break)))))))))
        (:then_2
          (CallFunction|UpdateTiles))))))

(event Custom|UpdateTiles
  (for (_array_element _array_index) (Variables|Default|GetHexes)
    (Development|PrintString (Utilities|String|ToString(Integer) _array_index))
    (Utilities|IsValid (Variables|/Game/Games/Neuroshima/Blueprints/NeuroBoardHex.NeuroBoardHex_C|GetTile _array_element)
      (:Is%20Valid
        (Class|Actor|AttachRootComponentto (Variables|/Game/Games/Neuroshima/Blueprints/NeuroBoardHex.NeuroBoardHex_C|GetTile _array_element) _array_element "Tile" "SnapToTarget" true)
        (Development|PrintText (Variables|/Script/UnrealGames.UGCard|GetCardName (Variables|/Game/Games/Neuroshima/Blueprints/NeuroBoardHex.NeuroBoardHex_C|GetTile _array_element))))
      (:Is%20Not%20Valid
        (Development|PrintString "nada")))))

(event Custom|ClearOutdated
  (for _array_element (Variables|Default|GetHexes)
    (Utilities|IsValid (Variables|/Game/Games/Neuroshima/Blueprints/NeuroBoardHex.NeuroBoardHex_C|GetTile _array_element)
      (:Is%20Valid
        (if (== (Utilities|Array|FindItem (Variables|/Script/UnrealGames.UGCardGroup|GetCards (Class|UGCardGroupVizComponent|GetGroup (Variables|Default|GetUGCardGroupViz))) (Variables|/Game/Games/Neuroshima/Blueprints/NeuroBoardHex.NeuroBoardHex_C|GetTile _array_element)) -1)
          (Variables|/Game/Games/Neuroshima/Blueprints/NeuroBoardHex.NeuroBoardHex_C|SetTile _array_element 0))))))

(event EventBeginPlay
  (Variables|Default|SetHexes (Utilities|Array|MakeArray (Variables|Default|GetNeuroBoardHex0) (Variables|Default|GetNeuroBoardHex1) (Variables|Default|GetNeuroBoardHex2))))

(fn ConstructionScript)