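; NeuroPS is a per-player Blueprint for the Neuroshima board game that rotates a tile to follow the mouse cursor.
; InputRotate stores the tile and opens a Tick-driven gate, which nothing here closes.
; Each tick projects the cursor ray onto a plane through the tile, derives a yaw from that point, and snaps it to one of six 60-degree steps.
; The tile's board then applies the updated rotation.
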(event Custom|InputRotate
  (params (Tile :type Neuro%20Base%20Tile%20Object%20Reference))
  (bind _returnvalue (Class|UGPS|GetOwningPlayerController))
  (bind (_locationx _locationy) (Game|Player|GetMousePosition _returnvalue))
  (bind _returnvalue_2 (Math|Vector2D|MakeVector2D _locationx _locationy))
  (bind (_worldposition _worlddirection) (Class|GameplayStatics|DeprojectScreentoWorld _returnvalue _returnvalue_2))
  (Variables|Default|SetRotatingTile Tile)
  (Utilities|FlowControl|Gate true) ; enters at Open
)

(event EventBeginPlay)

(event EventTick
  (params (DeltaSeconds :type Float%20%28single-precision%29))
  (bind _returnvalue (Class|UGPS|GetOwningPlayerController))
  (bind _rotatingtile (Variables|Default|GetRotatingTile))
  (bind _rotatingtile_2 (Variables|Default|GetRotatingTile))
  (bind (_locationx _locationy) (Game|Player|GetMousePosition _returnvalue))
  (bind _returnvalue_2 (Transformation|GetActorTransform _rotatingtile_2))
  (bind _returnvalue_3 (Math|Vector2D|MakeVector2D _locationx _locationy))
  (bind (_location _rotation) (Math|Transform|BreakTransform _returnvalue_2))
  (bind (_worldposition _worlddirection) (Class|GameplayStatics|DeprojectScreentoWorld _returnvalue _returnvalue_3))
  (Utilities|FlowControl|Gate true
    (:Exit
      (Utilities|IsValid _returnvalue
        (:Is%20Valid
          (Variables|/Game/Games/Neuroshima/Blueprints/Tile/AbstractClasses/NeuroBaseTile.NeuroBaseTile_C|SetRotation _rotatingtile (|(((floor(((((round(Angle))+720)%360)/60.000000)))+5)%6) (.Yaw (Math|Rotator|BreakRotator (Math|Conversions|RotationFromXVector (- (- (Class|UGFunctionLibrary|ProjectPointontoPlaneParallertoDirection _worldposition _location (Math|Rotator|GetRotationXVector (Math|Rotator|CombineRotators _rotation "90.000000, 0, 0")) _worlddirection) _location) (Math|Rotator|GetRotationXVector (Transformation|GetActorRotation (Default|GetBoard (Variables|Default|GetRotatingTile))))))))))
          (Default|UpdateTileRotation (Default|GetBoard _rotatingtile) _rotatingtile))))))

(fn ConstructionScript
  (|CallParentFunction))