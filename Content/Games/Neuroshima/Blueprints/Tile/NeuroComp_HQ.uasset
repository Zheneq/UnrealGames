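; NeuroComp_HQ is a tile component for Neuroshima that marks an HQ tile and displays its army's HP.
; Init casts the owner to NeuroBaseTile, caches it, and writes the army's HP to the tile's text render, skipping the visual when the component is temporal.
; It returns false only if the owner cast fails, and the HP text is set only during Init.
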(event EventBeginPlay)

(event EventTick
  (params (DeltaSeconds :type Float%20%28single-precision%29)))

(fn Init
  (bind _asneuro_base_tile (Utilities|Casting|CastToNeuroBaseTile (Components|GetOwner))
    (:then
      (Variables|Default|SetTile _asneuro_base_tile)
      (if (Variables|Default|GetIsTemporal) ; Not visualizing the component if it's temporal.
        (return true)
        (else
          (Rendering|Components|TextRender|SetText (Variables|/Game/Games/Neuroshima/Blueprints/Tile/AbstractClasses/NeuroBaseTile.NeuroBaseTile_C|GetTextRender (Variables|Default|GetTile)) (Utilities|Text|ToText(Integer) (Variables|/Game/Games/Neuroshima/Blueprints/NeuroArmy.NeuroArmy_C|GetHP (Variables|/Game/Games/Neuroshima/Blueprints/Tile/AbstractClasses/NeuroBaseTile.NeuroBaseTile_C|GetArmy (Variables|Default|GetTile))) false))
          (return true))))
    (:CastFailed
      (return false))))