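; Ranged attack component for Neuroshima hex tiles, holding an attack power for each direction.
; Init adds direction meshes scaled in count by power on non-temporal instances, and GetConsumedWidth reports the width used per direction.
; GiveDamage walks outward hex by hex along each powered direction, skipping empty hexes and tiles that do not accept the damage, until one does or the board ends.
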(event EventBeginPlay)

(event EventTick
  (params (DeltaSeconds :type Float%20%28single-precision%29)))

(fn Init
  (bind _success (|CallParentFunction))
  (if (Variables|Default|GetIsTemporal)
    _
    (else
      (for (_array_element _array_index) (Variables|Neuroshima|GetAttackPower)
        (CallFunction|AddMesh _array_index _array_element))))
  (return _success))

(fn GetConsumedWidth
  (bind _result (LocalVariables|GetResult))
  (for _array_element (Variables|Neuroshima|GetAttackPower)
    (if (Math|Conversions|ToBoolean(Integer) _array_element)
      (Utilities|Array|Add _result (|((N+0.500000)*{B292AAA3-45A1-1459-C0EE-CB977D3EB0F9}) _array_element))
      (else
        (Utilities|Array|Add _result 0.0))))
  (return (LocalVariables|GetResult)))

(fn GiveDamage
  (bind _tile (Variables|Default|GetTile))
  (bind _boardhex (Variables|/Game/Games/Neuroshima/Blueprints/Tile/AbstractClasses/NeuroBaseTile.NeuroBaseTile_C|GetBoardHex _tile))
  (|CallParentFunction)
  (Utilities|IsValid _boardhex
    (:Is%20Valid
      (for (_array_element _array_index) (Variables|Neuroshima|GetAttackPower)
        (if (> _array_element 0)
          (bind _output_get (LocalVariables|SetTargetedHex (Utilities|Array|Get(acopy) (Variables|/Game/Games/Neuroshima/Blueprints/NeuroBoardHex.NeuroBoardHex_C|GetNeighbours _boardhex) _array_index)))
          (Utilities|IsValid _output_get :!label _label
            (:Is%20Valid
              (Utilities|IsValid (Variables|/Game/Games/Neuroshima/Blueprints/NeuroBoardHex.NeuroBoardHex_C|GetTile _output_get)
                (:Is%20Valid
                  (bind _damagetaken (Default|NeuroDamage (Variables|/Game/Games/Neuroshima/Blueprints/NeuroBoardHex.NeuroBoardHex_C|GetTile _output_get) self _array_element))
                  (if (not _damagetaken)
                    (LocalVariables|SetTargetedHex (Default|GetNeighbour (LocalVariables|GetTargetedHex) _array_index) :!label _label_2)
                    (goto _label)))
                (:Is%20Not%20Valid
                  (goto _label_2)))))))
      (return true))
    (:Is%20Not%20Valid
      (Development|PrintString "Error: Tile not on the board is attempting to attack!" true true "(R=1.000000,G=0.000000,B=0.000000,A=1.000000)")
      (return false))))