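; Ranged attack component for Neuroshima tiles that lets the owning player pick which target in the line of fire to hit.
; FindTargets walks every hex along AttackDirection, using zero-value NeuroDamage calls to collect valid targets without stopping at the first.
; Attack offers these through ChooseTile, and Chosen passes the pick to GiveDamage, retrying if invalid.
; Init adds meshes and a Sharpshooter marker; BeginPlay warns if Ranged is also present.
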(event EventAttack
  (if (Variables|Default|GetIsInactive)
    (CallFunction|FindTargets)
    (Default|ChooseTile (Variables|/Game/Games/Neuroshima/Blueprints/NeuroArmy.NeuroArmy_C|GetOwningPlayer (Variables|/Game/Games/Neuroshima/Blueprints/Tile/AbstractClasses/NeuroBaseTile.NeuroBaseTile_C|GetArmy (Variables|Default|GetTile))) (Variables|NeuroGame|GetPossibleTargets) 1 self)
    (Variables|NeuroGame|SetPendingChoice true)))

(event EventBeginPlay
  (bind _tile (Variables|Default|GetTile))
  (if (> (Utilities|Array|Length (Actor|GetComponentsByClass _tile "/Game/Games/Neuroshima/Blueprints/Tile/NeuroComp_Ranged.NeuroComp_Ranged_C")) 0)
    (Development|PrintText (Utilities|Text|FormatText "WARNING: '{Tile}' has both Ranged attack and Sharpshooter. That may look confusing." (Variables|/Game/Games/Neuroshima/Blueprints/Tile/AbstractClasses/NeuroBaseTile.NeuroBaseTile_C|GetName _tile)) true true "(R=0.000000,G=0.660000,B=1.000000,A=1.000000)" 1e+01)))

(event EventChosen
  (params (Tiles :type Array%20of%20Neuro%20Base%20Tile%20Object%20References))
  (bind _item (Utilities|Array|Get(acopy) Tiles))
  (if (>= (Utilities|Array|FindItem (Variables|NeuroGame|GetPossibleTargets) _item) 0)
    (Variables|NeuroGame|SetTarget _item)
    (CallFunction|GiveDamage)
    (else
      (Development|PrintString "WARNING: Sharpshooter attack failed.")
      (CallFunction|Attack))))

(fn FindTargets
  (bind _tile (Variables|Default|GetTile))
  (bind _attackdirection (Variables|Neuroshima|GetAttackDirection))
  (bind _boardhex (Variables|/Game/Games/Neuroshima/Blueprints/Tile/AbstractClasses/NeuroBaseTile.NeuroBaseTile_C|GetBoardHex _tile))
  (Utilities|Array|Clear (Variables|NeuroGame|GetPossibleTargets))
  (Utilities|IsValid _boardhex
    (:Is%20Valid
      (if (> (Variables|Neuroshima|GetAttackPower) 0)
        (bind _output_get (LocalVariables|SetTargetedHex (Utilities|Array|Get(acopy) (Variables|/Game/Games/Neuroshima/Blueprints/NeuroBoardHex.NeuroBoardHex_C|GetNeighbours _boardhex) _attackdirection)))
        (Utilities|IsValid _output_get :!label _label
          (:Is%20Valid
            (Utilities|IsValid (Variables|/Game/Games/Neuroshima/Blueprints/NeuroBoardHex.NeuroBoardHex_C|GetTile _output_get)
              (:Is%20Valid
                (bind _damagetaken (Default|NeuroDamage (Variables|/Game/Games/Neuroshima/Blueprints/NeuroBoardHex.NeuroBoardHex_C|GetTile _output_get) self))
                (if _damagetaken
                  (Utilities|Array|Add (Variables|NeuroGame|GetPossibleTargets) (Variables|/Game/Games/Neuroshima/Blueprints/NeuroBoardHex.NeuroBoardHex_C|GetTile _output_get))))
              (:Is%20Not%20Valid
                _))
            (LocalVariables|SetTargetedHex (Default|GetNeighbour (LocalVariables|GetTargetedHex) _attackdirection))
            (goto _label)))))
    (:Is%20Not%20Valid
      (Development|PrintString "Error: Tile not on the board is attempting to attack!" true true "(R=1.000000,G=0.000000,B=0.000000,A=1.000000)"))))

(fn GiveDamage
  (|CallParentFunction)
  (bind _damagetaken (Default|NeuroDamage (Variables|NeuroGame|GetTarget)))
  (return _damagetaken))

(fn Init
  (bind _success (|CallParentFunction))
  (if (Variables|Default|GetIsTemporal)
    _
    (else
      (CallFunction|AddMesh (Variables|Neuroshima|GetAttackDirection) (Variables|Neuroshima|GetAttackPower))
      (Default|AddMarker (Variables|Default|GetTile) "/Game/Games/Neuroshima/Meshes/Markers/NeuroHex_Marker_Sharpshooter.NeuroHex_Marker_Sharpshooter")))
  (return _success))

(fn GetConsumedWidth
  (bind _output_get (LocalVariables|SetResult (Utilities|Array|MakeArray 0.0 0.0 0.0 0.0 0.0 0.0)))
  (if (Math|Conversions|ToBoolean(Integer) (Variables|Neuroshima|GetAttackPower))
    (Utilities|Array|SetArrayElem _output_get (Variables|Neuroshima|GetAttackDirection) (|(({603504E7-4CD9-0D19-7BD3-D3B7194B0B5C}+0.500000)*{B292AAA3-45A1-1459-C0EE-CB977D3EB0F9}))))
  (return (LocalVariables|GetResult)))