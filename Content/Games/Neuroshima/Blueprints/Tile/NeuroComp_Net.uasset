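; Tile component for the Neuroshima board game's Net ability, which applies a net effect to neighbouring tiles in its flagged directions.
; On init it adds a mesh for each net direction unless the component is temporal.
; When the tile moves, it removes its own effects around the previous hex and captures neighbours around the new one.
; A looping macro shared by release and capture yields valid neighbour tiles under the net.
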(event Custom|ReleaseDisabled
  (params (Hex :type Neuro%20Board%20Hex%20Object%20Reference))
  (bind _tile (Utilities|ForEachValidNeighbourUnderNet Hex)
    (:Is%20Valid
      (Default|RemoveEffect _tile "/Game/Games/Neuroshima/Blueprints/Effects/NeuroEffect_Net.NeuroEffect_Net_C" self))))

(event Custom|Capture
  (bind _tile (Utilities|ForEachValidNeighbourUnderNet (Variables|/Game/Games/Neuroshima/Blueprints/Tile/AbstractClasses/NeuroBaseTile.NeuroBaseTile_C|GetBoardHex (Variables|Default|GetTile)))
    (:Is%20Valid
      (CallFunction|AddEffecttoTile "/Game/Games/Neuroshima/Blueprints/Effects/NeuroEffect_Net.NeuroEffect_Net_C" _tile))))

(event EventOnTileMoved
  (params (From :type Neuro%20Board%20Hex%20Object%20Reference))
  (|CallParentFunction From)
  (CallFunction|ReleaseDisabled From)
  (CallFunction|Capture))

(fn Init
  (bind _success (|CallParentFunction))
  (if (Variables|Default|GetIsTemporal)
    _
    (else
      (for (_array_element _array_index) (Variables|Default|GetNetDirections)
        (if _array_element
          (CallFunction|AddMesh _array_index 1)))))
  (return _success))