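; Test tile actor for Neuroshima that exercises tile rotation and visualizes the math behind it.
; On BeginPlay it passes itself to InputRotate on the first player's NeuroPS player state, printing an error if that cast fails.
; Every tick it projects the mouse ray onto a plane through the mesh, oriented from the actor's rotation, then draws debug lines to that point and along the plane normal.
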(event EventBeginPlay
  (bind _asneuro_ps (Utilities|Casting|CastToNeuroPS (Variables|/Script/Engine.Controller|GetPlayerState (Game|GetPlayerController 0)))
    (:then
      (Default|InputRotate _asneuro_ps self))
    (:CastFailed
      (Development|PrintString "TestRotaatingTile: No NueroPS!!" true true "(R=0.000000,G=0.660000,B=1.000000,A=1.000000)" 2e+01))))

(event EventTick
  (params (DeltaSeconds :type Float%20%28single-precision%29))
  (bind _returnvalue (Game|GetPlayerController 0))
  (bind _returnvalue_2 (Transformation|GetActorRotation))
  (bind _mesh (Variables|Character|GetMesh))
  (bind _returnvalue_3 (Math|Rotator|CombineRotators "90.000000, 0, 0" _returnvalue_2))
  (bind (_locationx _locationy) (Game|Player|GetMousePosition _returnvalue))
  (bind _returnvalue_4 (Transformation|GetWorldTransform _mesh))
  (bind _returnvalue_5 (Math|Vector2D|MakeVector2D _locationx _locationy))
  (bind _location (Math|Transform|BreakTransform _returnvalue_4))
  (bind _returnvalue_6 (Math|Rotator|GetRotationXVector _returnvalue_3))
  (bind (_worldposition _worlddirection) (Class|GameplayStatics|DeprojectScreentoWorld _returnvalue _returnvalue_5))
  (Rendering|Debug|DrawDebugLine _location (Class|UGFunctionLibrary|ProjectPointontoPlaneParallertoDirection _worldposition _location _returnvalue_6 _worlddirection) "(R=0.109658,G=0.004004,B=0.570000,A=1.000000)" 0.05 5.0)
  (Rendering|Debug|DrawDebugLine _location (+ _location (* _returnvalue_6 1e+02)) "(R=0.570000,G=0.000000,B=0.018444,A=1.000000)" 0.05 5.0))

(fn ConstructionScript
  (|CallParentFunction))