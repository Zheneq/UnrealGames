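; Game logic for the Neuroshima tile game, setting up and resetting each player's tiles through a card manager.
; PreInitGame spawns the UGCardManager, creates a public Table group plus per-player Hand, Army and Discard groups, then spawns each army's tiles far off-origin and registers them as cards.
; PreInitRound restarts the manager, and InitPlayer shuffles that player's secret Army pile.
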(event EventPreInitRound
  ;[1 1 1] Reset Round
  (Class|UGCardManager|Restart (Variables|NeuroGame|GetCardManager)))

(event EventPreInitGame
  ;[1 1 1] Init CardManager
  (bind _returnvalue (Game|SpawnActorfromClass "/Script/UnrealGames.UGCardManager" (Math|Transform|MakeTransform "0, 0, 0") "AlwaysSpawn" self 0))
  (Variables|NeuroGame|SetCardManager _returnvalue)
  (Utilities|FlowControl|Sequence
    (:then_0
      (Class|UGCardManager|CreateGroup (Variables|NeuroGame|GetCardManager) 0 "Table" "CGP_Public"))
    (:then_1
      (for _array_element (Variables|Default|GetPlayers)
        (bind _asneuro_ps (Utilities|Casting|CastToNeuroPS _array_element))
        (Utilities|FlowControl|Sequence
          (:then_0
            (Class|UGCardManager|CreateGroup (Variables|NeuroGame|GetCardManager) _asneuro_ps "Hand" "CGP_Public")
            (Class|UGCardManager|CreateGroup (Variables|NeuroGame|GetCardManager) _asneuro_ps "Army" "CGP_Secret")
            (Class|UGCardManager|CreateGroup (Variables|NeuroGame|GetCardManager) _asneuro_ps "Discard" "CGP_Secret"))
          (:then_1
            (for _array_element_2 (Variables|/Game/Games/Neuroshima/Blueprints/NeuroArmy.NeuroArmy_C|GetTiles (Variables|/Game/Games/Neuroshima/Blueprints/NeuroPS.NeuroPS_C|GetArmy _asneuro_ps))
              (bind _returnvalue_2 (Game|SpawnActorfromClass _array_element_2 (Math|Transform|MakeTransform "10000.000000,10000.000000,10000.000000") "Undefined" 0 false 0))
              (Class|UGCardManager|RegisterCard (Variables|NeuroGame|GetCardManager) _returnvalue_2 _asneuro_ps "Army"))))))))

(event EventInitPlayer
  (params (Index :type Integer) (Player :type UGPS%20BP%20Object%20Reference))
  ;[1 1 1] Init Player
  (bind _asneuro_ps (Utilities|Casting|CastToNeuroPS Player))
  (Class|UGCardManager|Shuffle (Variables|NeuroGame|GetCardManager) _asneuro_ps "Army"))

(fn ConstructionScript
  (|CallParentFunction))