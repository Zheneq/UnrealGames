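; A single hex cell of the Neuroshima game board, holding a Tile, a FoundationTile and six directional neighbour links.
; Reset rebuilds the neighbour array and clears both tiles, while IsEmpty checks only the main Tile.
; GetNeighbour lets the first tile NeuroComp implementing NeuroIF_Neighbour override the result, otherwise returning the stored link.
; With DrawDebug on, Tick draws the hex name and colour-coded, numbered lines toward each valid neighbour.
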(event Custom|Reset
  (bind _neighbours (Variables|Neuroshima|GetNeighbours))
  (Utilities|Array|Clear _neighbours)
  (for _index (range 1 6)
    (Utilities|Array|Add _neighbours 0))
  (Variables|Neuroshima|SetTile 0)
  (Variables|Neuroshima|SetFoundationTile 0))

(event EventTick
  (params (DeltaSeconds :type Float%20%28single-precision%29))
  (bind _returnvalue (Transformation|GetWorldLocation))
  (if (Variables|NeuroDebug|GetDrawDebug)
    (Rendering|Debug|DrawDebugString (+ (Transformation|GetWorldLocation) "0, 0,20.000000") (Utilities|String|Append "== " (Utilities|GetObjectName self) " ==") 0 "(R=0.466123,G=1.000000,B=0.142912,A=1.000000)" 1.0)
    (for (_array_element _array_index) (Variables|Neuroshima|GetNeighbours)
      (Utilities|IsValid _array_element
        (:Is%20Valid
          (Rendering|Debug|DrawDebugLine (+ _returnvalue "0, 0,10.000000") (+ (+ _returnvalue (* (- (Transformation|GetWorldLocation _array_element) _returnvalue) 0.4)) "0, 0,10.000000") (Utilities|Struct|MakeLinearColor (* _array_index 0.5) (* (- _array_index 2) 0.5) (* (- _array_index 4) 0.5) 0.0) 1.0 2.0)
          (Rendering|Debug|DrawDebugString (+ (+ (+ _returnvalue (* (- (Transformation|GetWorldLocation _array_element) _returnvalue) 0.4)) "0, 0,10.000000") "0, 0, 0") (Utilities|String|ToString(Integer) _array_index) 0 (Utilities|Struct|MakeLinearColor (* _array_index 0.5) (* (- _array_index 2) 0.5) (* (- _array_index 4) 0.5) 0.0) 1.0))))))

(fn IsEmpty
  (return (not (Utilities|IsValid (Variables|Neuroshima|GetTile)))))

(fn GetNeighbour
  (params (Direction :type Integer))
  (bind _tile (Variables|Neuroshima|GetTile))
  (Utilities|IsValid _tile
    (:Is%20Valid
      (for _array_element (Actor|GetComponentsByClass _tile "/Game/Games/Neuroshima/Blueprints/Tile/AbstractClasses/NeuroComp.NeuroComp_C")
        (if (Utilities|DoesObjectImplementInterface _array_element "/Game/Games/Neuroshima/Blueprints/NeuroIF_Neighbour.NeuroIF_Neighbour_C")
          (bind _hex (Class|NeuroIFNeighbour|GetNeighbour(Message) _array_element Direction))
          (return _hex))))
    (:Is%20Not%20Valid
      _))
  (return (Utilities|Array|Get(acopy) (Variables|Neuroshima|GetNeighbours) Direction)))