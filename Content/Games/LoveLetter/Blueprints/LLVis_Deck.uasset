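; Love Letter deck visualizer that shows a card group as a physical pile of face-down cards.
; On each visualizer update it compares the group's card count to the visible count, spawning pooled card actors only when short.
; When the count grows, cards are restacked at the spawn point with random yaw, dropped with physics, then frozen after a short delay.
; Surplus cards are hidden and made non-solid rather than destroyed.
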(event UpdateVisualizer(UGCardGroupViz)
  (bind _renderedcards (Variables|Default|GetRenderedCards))
  (bind _spawnpoint (Variables|Default|GetSpawnPoint))
  (bind _ugcardgroupviz (Variables|Default|GetUGCardGroupViz))
  (bind _ugcardgroupviz_2 (Variables|Default|GetUGCardGroupViz))
  (bind _renderedcards_2 (Variables|Default|GetRenderedCards))
  (bind _returnvalue (Utilities|Array|Length _renderedcards_2))
  (bind _returnvalue_2 (Transformation|GetWorldTransform _spawnpoint))
  (bind _info (Variables|/Script/UnrealGames.UGCardGroupVizComponent|GetInfo _ugcardgroupviz_2))
  (bind _info_2 (Variables|/Script/UnrealGames.UGCardGroupVizComponent|GetInfo _ugcardgroupviz))
  (bind (_location _rotation _scale) (Math|Transform|BreakTransform _returnvalue_2))
  (bind _cardcount (Variables|/Script/UnrealGames.UGCardGroupInfo|GetCardCount _info))
  (bind _cardcount_2 (Variables|/Script/UnrealGames.UGCardGroupInfo|GetCardCount _info_2))
  (bind (_roll _pitch _yaw) (Math|Rotator|BreakRotator _rotation))
  (Utilities|IsValid _info_2
    (:Is%20Valid
      (Development|PrintText (Utilities|Text|FormatText "Deck: {0}/{1}" (Utilities|Text|ToText(Integer) (Variables|Default|GetVisibleCards)) (Utilities|Text|ToText(Integer) _cardcount_2)) false)
      (bind _output_get (Variables|Default|SetCardsDifference (- _cardcount_2 (Variables|Default|GetVisibleCards))))
      (if (!= _output_get 0)
        (if (> _output_get 0)
          (if (> _cardcount _returnvalue)
            (bind _output_get_2 (Variables|Default|SetCardsToSpawn (- _cardcount _returnvalue)))
            (for _index (range 1 _output_get_2)
              (bind _returnvalue_3 (Game|SpawnActorfromClass "/Game/Generic/UGPhysicalCard.UGPhysicalCard_C" (Math|Transform|MakeTransform "0, 0, 0") "Undefined" self "/Game/Games/LoveLetter/Materials/M_LLCard_Back.M_LLCard_Back" "/Game/Games/LoveLetter/Materials/M_LLCard_Back.M_LLCard_Back" 0 false (Variables|Default|GetUGCardGroupViz)))
              (Utilities|Array|Add (Variables|Default|GetRenderedCards) _returnvalue_3)))
          (for _index_2 (range 0 (- (Variables|/Script/UnrealGames.UGCardGroupInfo|GetCardCount (Variables|/Script/UnrealGames.UGCardGroupVizComponent|GetInfo (Variables|Default|GetUGCardGroupViz))) 1))
            (Transformation|SetActorTransform (Utilities|Array|Get(acopy) (Variables|Default|GetRenderedCards) _index_2) (Math|Transform|MakeTransform (+ _location (* (Math|Vector|MakeVector 0.0 0.0 5.0) _index_2)) (Math|Rotator|MakeRotator _roll _pitch (+ _yaw (Math|Random|RandomFloatinRange -5.0 5.0))) _scale) false true)
            (Default|SetPhysics (Utilities|Array|Get(acopy) (Variables|Default|GetRenderedCards) _index_2) true true true))
          (Utilities|FlowControl|Sequence
            (:then_0
              (bind _output_get_3 (Variables|Default|SetVisibleCards (Variables|/Script/UnrealGames.UGCardGroupInfo|GetCardCount (Variables|/Script/UnrealGames.UGCardGroupVizComponent|GetInfo (Variables|Default|GetUGCardGroupViz))) :!label _label))
              (for _index_3 (range _output_get_3 (Utilities|Array|LastIndex _renderedcards))
                (Default|SetPhysics (Utilities|Array|Get(acopy) _renderedcards _index_3) false false false)))
            (:then_1
              (Utilities|FlowControl|Delay 1.5)
              (for _array_element (Variables|Default|GetRenderedCards)
                (Default|SetSimulatesPhysics _array_element false))))
          (else
            (goto _label)))))))

(fn ConstructionScript)