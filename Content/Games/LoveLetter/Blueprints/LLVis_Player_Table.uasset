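; Card group visualizer for Love Letter that shows a player's table cards as physical card actors.
; On update, it spawns only newly added cards in a scaled row from the spawn point, with a dynamic material indexed by card value for the front.
; Cards spawn simulating physics, then all freeze after a short delay.
; If the group shrinks, it destroys and rebuilds every card; reset just clears them.
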(event UpdateVisualizer(UGCardGroupViz)
  (bind _renderedcards (Variables|Default|GetRenderedCards))
  (bind _renderedcards_2 (Variables|Default|GetRenderedCards))
  (bind _ugcardgroupviz (Variables|Default|GetUGCardGroupViz))
  (bind _cardspawnpoint (Variables|Default|GetCardSpawnPoint))
  (bind _returnvalue (Utilities|Array|Length _renderedcards))
  (bind _returnvalue_2 (Class|UGCardGroupVizComponent|GetGroup _ugcardgroupviz))
  (bind _returnvalue_3 (Transformation|GetWorldTransform _cardspawnpoint))
  (bind (_location _rotation _scale) (Math|Transform|BreakTransform _returnvalue_3))
  (bind _cards (Variables|/Script/UnrealGames.UGCardGroup|GetCards _returnvalue_2))
  (bind _returnvalue_4 (Utilities|Array|Length _cards))
  (Utilities|IsValid _returnvalue_2 :!label _label
    (:Is%20Valid
      (if (> _returnvalue_4 _returnvalue)
        (bind _output_get (Variables|Default|SetTempInt _returnvalue))
        (for _index (range _output_get (Utilities|Array|LastIndex _cards))
          (bind _asllbase_card (Utilities|Casting|CastToLLBaseCard (Utilities|Array|Get(acopy) _cards _index)))
          (bind _returnvalue_5 (Rendering|Material|CreateDynamicMaterialInstance "/Game/Games/LoveLetter/Materials/M_LLCard_Back.M_LLCard_Back" :!class /Script/Engine.KismetMaterialLibrary))
          (Rendering|Material|SetScalarParameterValue _returnvalue_5 "Card Index" (Math|Conversions|ToFloat(Integer) (- (Variables|/Game/Games/LoveLetter/Blueprints/LLBaseCard.LLBaseCard_C|GetValue _asllbase_card) 1)) :!class /Script/Engine.MaterialInstanceDynamic)
          (bind _returnvalue_6 (Game|SpawnActorfromClass "/Game/Generic/UGPhysicalCard.UGPhysicalCard_C" (Math|Transform|MakeTransform (+ (Math|Vector|RotateVector (* (Variables|Default|GetShiftPerCard) (* _index (.X (Math|Vector|BreakVector (Transformation|GetActorScale3D))))) _rotation) _location) _rotation _scale) "Undefined" self _returnvalue_5 "/Game/Games/LoveLetter/Materials/M_LLCard_Back.M_LLCard_Back" 0 true (Variables|Default|GetUGCardGroupViz)))
          (Utilities|Array|Add (Variables|Default|GetRenderedCards) _returnvalue_6))
        (Utilities|FlowControl|Delay 1.0)
        (for _array_element (Variables|Default|GetRenderedCards)
          (Default|SetPhysics _array_element false true true))
        (elif (< _returnvalue_4 _returnvalue)
          (Utilities|FlowControl|Sequence
            (:then_0
              (for _array_element_2 _renderedcards_2
                (Actor|DestroyActor _array_element_2))
              (Utilities|Array|Clear _renderedcards_2))
            (:then_1
              (goto _label))))))))

(event EventOnReset
  (bind _renderedcards (Variables|Default|GetRenderedCards))
  (for _array_element _renderedcards
    (Actor|DestroyActor _array_element))
  (Utilities|Array|Clear _renderedcards))

(fn ConstructionScript)