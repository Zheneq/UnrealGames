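; Love Letter card 5, the Prince, which makes a target player discard their card and draw a replacement.
; Its Card event prints a message naming both players, then casts the current game to GameLoveLetter and calls Discard and Draw on the other player.
; The construction script only calls its parent.
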(event EventCard
  (params (Player :type LLPS%20Object%20Reference) (OtherPlayer :type LLPS%20Object%20Reference) (Value :type Integer))
  (Development|PrintText (Utilities|Text|FormatText "{0} makes {1} discard their card." (Utilities|Text|ToText(String) (Variables|/Script/Engine.PlayerState|GetPlayerName Player)) (Utilities|Text|ToText(String) (Variables|/Script/Engine.PlayerState|GetPlayerName OtherPlayer))) false)
  (bind _asgame_love_letter (Utilities|Casting|CastToGameLoveLetter (Class|UGFunctionLibrary|GetGame)))
  (Default|Discard _asgame_love_letter OtherPlayer)
  (Default|Draw _asgame_love_letter OtherPlayer))

(fn ConstructionScript
  (|CallParentFunction))