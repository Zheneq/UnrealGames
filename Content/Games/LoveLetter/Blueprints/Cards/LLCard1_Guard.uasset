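; Guard card for the Love Letter game, which lets a player guess the value of another player's hand card.
; Its Card event announces the attack, then reads the first card in the target's Hand group through CardManager.
; A match with that card's Value makes the target lose the round through GameLoveLetter.
; A miss prints a failure and writes a denial message to the game log.
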(event EventCard
  (params (Player :type LLPS%20Object%20Reference) (OtherPlayer :type LLPS%20Object%20Reference) (Value :type Integer))
  (Development|PrintText (Utilities|Text|FormatText "{0} attacks {1} with Guard ({2})" (Utilities|Text|ToText(String) (Variables|/Script/Engine.PlayerState|GetPlayerName Player)) (Utilities|Text|ToText(String) (Variables|/Script/Engine.PlayerState|GetPlayerName OtherPlayer)) (Utilities|Text|ToText(Integer) Value)) false)
  (bind _asllbase_card (Utilities|Casting|CastToLLBaseCard (Utilities|Array|Get(acopy) (Variables|/Script/UnrealGames.UGCardGroup|GetCards (Class|UGCardManager|GetGroup (Variables|Default|GetCardManager) OtherPlayer "Hand")))))
  (bind _asgame_love_letter (Utilities|Casting|CastToGameLoveLetter (Class|UGFunctionLibrary|GetGame)))
  (if (== (Variables|/Game/Games/LoveLetter/Blueprints/LLBaseCard.LLBaseCard_C|GetValue _asllbase_card) Value)
    (Class|UGGame|LoseRound _asgame_love_letter OtherPlayer)
    (Development|PrintText "Well done!" false)
    (else
      (Development|PrintText "Failed." false)
      (Class|UGGame|Log _asgame_love_letter (Utilities|Text|FormatText "{Player} doesn't think so." (Utilities|Text|ToText(String) (Variables|/Script/Engine.PlayerState|GetPlayerName OtherPlayer)))))))

(fn ConstructionScript
  (|CallParentFunction))