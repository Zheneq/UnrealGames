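; Love Letter King card (card 6) Blueprint that makes the player exchange hand cards with another chosen player.
; Its Card event prints the exchange message with both player names, then swaps through CardManager.
; The other player's first Hand card is pushed onto the top of the player's Hand, then the player's bottom card is popped to the other player, so no temporary storage is needed.
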(event EventCard
  (params (Player :type LLPS%20Object%20Reference) (OtherPlayer :type LLPS%20Object%20Reference) (Value :type Integer))
  (Development|PrintText (Utilities|Text|FormatText "{0} exchanges card with {1}." (Utilities|Text|ToText(String) (Variables|/Script/Engine.PlayerState|GetPlayerName Player)) (Utilities|Text|ToText(String) (Variables|/Script/Engine.PlayerState|GetPlayerName OtherPlayer))) false)
  (Class|UGCardManager|PushTop (Variables|Default|GetCardManager) (Utilities|Array|Get(acopy) (Variables|/Script/UnrealGames.UGCardGroup|GetCards (Class|UGCardManager|GetGroup (Variables|Default|GetCardManager) OtherPlayer "Hand"))) Player "Hand")
  (Class|UGCardManager|PopBottom (Variables|Default|GetCardManager) "Hand" OtherPlayer "Hand" Player))

(fn ConstructionScript
  (|CallParentFunction))