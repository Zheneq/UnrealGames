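; Baron card for the Love Letter game, which compares the player's hand with a chosen opponent's and knocks out the lower one.
; When played, it calls Learn in both directions so each player learns the other's card, then compares the returned values.
; The loser is passed to LoseRound on GameLoveLetter, while a tie eliminates nobody.
; Each step is announced with printed text.
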(event EventCard
  (params (Player :type LLPS%20Object%20Reference) (OtherPlayer :type LLPS%20Object%20Reference) (Value :type Integer))
  (Development|PrintText (Utilities|Text|FormatText "{0} compares his hand with {1}'s one." (Utilities|Text|ToText(String) (Variables|/Script/Engine.PlayerState|GetPlayerName Player)) (Utilities|Text|ToText(String) (Variables|/Script/Engine.PlayerState|GetPlayerName OtherPlayer))) false)
  (Utilities|Casting|CastToLLBaseCard (Utilities|Array|Get(acopy) (Variables|/Script/UnrealGames.UGCardGroup|GetCards (Class|UGCardManager|GetGroup (Variables|Default|GetCardManager) Player "Hand"))))
  (bind _other_player_card (CallFunction|Learn OtherPlayer Player))
  (bind _other_player_card_2 (CallFunction|Learn Player OtherPlayer))
  (if (== _other_player_card _other_player_card_2)
    (Development|PrintText "It's a tie!" false)
    (else
      (bind _asgame_love_letter (Utilities|Casting|CastToGameLoveLetter (Class|UGFunctionLibrary|GetGame)))
      (if (> _other_player_card _other_player_card_2)
        (Class|UGGame|LoseRound _asgame_love_letter OtherPlayer)
        (Development|PrintText (Utilities|Text|FormatText "{0} lost." (Utilities|Text|ToText(String) (Variables|/Script/Engine.PlayerState|GetPlayerName OtherPlayer))) false)
        (else
          (Class|UGGame|LoseRound _asgame_love_letter Player)
          (Development|PrintText (Utilities|Text|FormatText "{0} committed suicide." (Utilities|Text|ToText(String) (Variables|/Script/Engine.PlayerState|GetPlayerName Player))) false))))))

(fn ConstructionScript
  (|CallParentFunction))