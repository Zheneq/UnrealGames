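; Base card Blueprint for Love Letter that handles playing a card from the local player's hand.
; A click checks turn, ownership and the rule blocking 5 or 6 beside a 7, then prompts via LLPC for target or value as needed.
; Choices re-enter ClientActivate until ServerActivate is called.
; Execute involves a Handmaid protection check, the empty Card effect hook and turn ending, while Learn reveals another player's hand to a player or bot.
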(event Custom|Chosen
  (params (OtherPlayer :type LLPS%20Object%20Reference) (Value :type Integer))
  (if (Variables|Default|GetPending%20User%20Choice)
    (Utilities|IsValid OtherPlayer
      (:Is%20Valid
        (Variables|Default|SetOther%20Player OtherPlayer))
      (:Is%20Not%20Valid
        _))
    (if (and (<= Value 8) (>= Value 2))
      (Variables|Default|SetOther%20Value Value))
    (CallFunction|ClientActivate)
    (else
      (Development|PrintText "Recieved unexpected choice." false))))

(event Custom|Activate
  (Variables|Default|SetOther%20Player 0)
  (Variables|Default|SetOther%20Value 0)
  (Variables|Default|SetPending%20User%20Choice true)
  (CallFunction|ClientActivate))

(event EventClicked
  (params (Key :type Key%20Structure :default "AnyKey"))
  (bind _group (Variables|Default|GetGroup))
  (Development|PrintText (Utilities|Text|FormatText "{Card} is clicked!" (Variables|Default|GetCardName)) false true "(R=0.062484,G=0.810000,B=0.000000,A=1.000000)" 1e+01)
  (bind _asllps (Utilities|Casting|CastToLLPS (Variables|/Script/Engine.Controller|GetPlayerState (Game|GetPlayerController 0))))
  (if (Math|Boolean|ANDBoolean (Utilities|IsValid _group) (== _asllps (Components|GetOwner _group)) (Utilities|Name|Equal(Name) (Variables|/Script/UnrealGames.UGCardGroup|GetCardGroupName _group) "Hand") (Variables|/Script/UnrealGames.UGPS|GetbMyTurn _asllps)) ; If it's a valid card in my hand
    (Utilities|IsAllowedtoActivate
      (:Allowed
        (CallFunction|Activate)))))

(fn ConstructionScript)

(fn ClientActivate
  (bind _self self)
  (bind _value (Variables|Default|GetValue))
  (bind _asllpc (Utilities|Casting|CastToLLPC (Game|GetPlayerController 0))
    (:then
      (switch int _value
        (:Default
          (Development|PrintText "Problems" false :!label _label)
          (return))
        (:0
          (goto _label))
        (:1
          (Utilities|FlowControl|Sequence
            (:then_0
              (if (not (Utilities|IsValid (Variables|Default|GetOther%20Player))) :!label _label_2
                (Default|ChoosePlayer _asllpc (== _value 5) _self)
                (return)))
            (:then_1
              (if (== (Variables|Default|GetOther%20Value) 0)
                (Default|ChooseValue _asllpc _self)
                (return)
                (else
                  (Default|ServerActivate _asllpc self (Variables|Default|GetOther%20Player) (Variables|Default|GetOther%20Value) :!label _label_3)
                  (Variables|Default|SetPending%20User%20Choice false)
                  (return))))))
        (:2
          (Utilities|FlowControl|Sequence :!label _label_4
            (:then_0
              (goto _label_2))
            (:then_1
              (goto _label_3))))
        (:3
          (goto _label_4))
        (:4
          (goto _label_3))
        (:5
          (goto _label_4))
        (:6
          (goto _label_4))
        (:7
          (goto _label_3))
        (:8
          (goto _label_3))))
    (:CastFailed
      (return))))

(fn AllowedtoActivate
  (Utilities|IsAllowedtoActivate
    (:Allowed
      (return true))
    (:Not%20Allowed
      (return false))))

(fn Execute
  (params (Player :type LLPS%20Object%20Reference) (OtherPlayer :type LLPS%20Object%20Reference) (Value :type Integer))
  (Utilities|FlowControl|Sequence
    (:then_0
      (if (Variables|Default|GetNeedsTarget)
        (Utilities|IsValid OtherPlayer
          (:Is%20Valid
            (if (Variables|/Game/Games/LoveLetter/Blueprints/LLPS.LLPS_C|GetProtected OtherPlayer)
              (Development|PrintText (Utilities|Text|FormatText "Failed. {0} is protected by Handmaid." (Utilities|Text|ToText(String) (Variables|/Script/Engine.PlayerState|GetPlayerName OtherPlayer))) false)
              (Utilities|FlowControl|Sequence
                (:then_0
                  (goto _label_2 Close))
                (:then_1
                  (bind _asgame_love_letter (Utilities|Casting|CastToGame_LoveLetter (Game|GetGameMode) :!label _label))
                  (Default|EndTurn _asgame_love_letter Player))))))))
    (:then_1
      (Utilities|FlowControl|Gate false :!label _label_2
        (:Exit
          (CallFunction|Card Player OtherPlayer Value)
          (goto _label))))))

(fn Card
  (params (Player :type LLPS%20Object%20Reference) (OtherPlayer :type LLPS%20Object%20Reference) (Value :type Integer))
  (return))

(fn Learn
  (params (Who :type LLPS%20Object%20Reference) (OtherPlayer :type LLPS%20Object%20Reference))
  (bind _controller (Default|GetController Who))
  (bind _asllbase_card (Utilities|Casting|CastToLLBaseCard (Utilities|Array|Get(acopy) (Variables|/Script/UnrealGames.UGCardGroup|GetCards (Class|UGCardManager|GetGroup (Variables|Default|GetCardManager) OtherPlayer "Hand"))))
    (:then
      (Utilities|FlowControl|Sequence
        (:then_0
          (bind _asllpc (Utilities|Casting|CastToLLPC _controller)
            (:then
              (Default|Learn _asllpc OtherPlayer (Variables|LLBaseCard_C|GetValue _asllbase_card)))
            (:CastFailed
              (bind _asllbot (Utilities|Casting|CastToLLBot _controller))
              (Default|Learn _asllbot OtherPlayer (Variables|LLBaseCard_C|GetValue _asllbase_card)))))
        (:then_1
          (return (Variables|LLBaseCard_C|GetValue _asllbase_card)))))
    (:CastFailed
      (return 0))))

(fn GetToolTip
  (return (Utilities|Text|FormatText "{group} - {card}" (Variables|/Script/UnrealGames.UGCardGroupInfo|GetGroupName (Variables|/Script/UnrealGames.UGCardGroup|GetInfo (Variables|Default|GetGroup))) (Variables|Default|GetCardName))))