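; GameLoveLetter is the game-rules Blueprint for a Love Letter card game, running rounds, turns and game-over.
; It spawns a UGCardManager with secret Deck and RB piles plus per-player Hand and Table groups bound to tagged visualizers.
; ExecuteCard validates turn, ownership and target before discarding and executing the card; discards add to RoundScore, and value 8 loses the round.
; GetWinners compares hand values, breaks ties by RoundScore, and lets the winner start next.
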(event EventInitRound
  (bind _cardmanager (Variables|LoveLetter|GetCardManager))
  ;[1 1 1] Init Round
  (Class|UGCardManager|Restart _cardmanager)
  (Class|UGCardManager|Shuffle _cardmanager 0 "Deck")
  (Class|UGCardManager|PopTop _cardmanager "Deck" 0 "RB"))

(event EventTurn
  ;[1 1 1] Game Turn
  (bind _asllps (Utilities|Casting|CastToLLPS (Class|UGGame|GetCurPlayer)))
  (Variables|/Game/Games/LoveLetter/Blueprints/LLPS.LLPS_C|SetProtected _asllps false)
  (CallFunction|Draw _asllps))

(event EventLost
  (params (Player :type UGPS%20Object%20Reference))
  ;[1 1 1] Lost
  (Class|UGGame|Log (Utilities|Text|FormatText "{Player} loses." (Utilities|Text|ToText(String) (Variables|/Script/Engine.PlayerState|GetPlayerName Player))))
  (bind _asllps (Utilities|Casting|CastToLLPS Player))
  (CallFunction|Discard _asllps))

(event EventGameOver
  ;[1 1 1] GameOver
  (|CallParentFunction)
  (bind _array_element (Utilities|Array|ForEachLoopwithBreak (Variables|Default|GetPlayers) :!label _label)
    (:LoopBody
      (if (Math|Float|NearlyEqual(Float) (Variables|/Script/Engine.PlayerState|GetScore _array_element) (Math|Conversions|ToFloat(Integer) (.outValue (Class|UGSettingsComponent|GetIntParam (Variables|Default|GetGameSettings) "WinScore"))) 0.4)
        (Variables|Default|SetWinnerOfTheGame _array_element)
        (goto _label Break)))
    (:Completed
      (Class|UGGame|Log (Utilities|Text|FormatText "And the winner is... {Winner}!" (Utilities|Text|ToText(String) (Variables|/Script/Engine.PlayerState|GetPlayerName (Variables|Default|GetWinnerOfTheGame))))))))

(event EventInitPlayer
  (params (Player :type UGPS%20Object%20Reference))
  ;[1 1 1] Init player
  (bind _asllps (Utilities|Casting|CastToLLPS Player))
  (Variables|/Game/Games/LoveLetter/Blueprints/LLPS.LLPS_C|SetRoundScore _asllps 0)
  (Variables|/Game/Games/LoveLetter/Blueprints/LLPS.LLPS_C|SetCardsDiscarded _asllps 0)
  (CallFunction|Draw _asllps))

(event EventInitGame
  (Utilities|FlowControl|Sequence
    (:then_0
      ;[1 1 1] Init CardManager
      (bind _returnvalue (Game|SpawnActorfromClass "/Script/UnrealGames.UGCardManager" (Math|Transform|MakeTransform "0, 0, 0") "AlwaysSpawn" self 0))
      (Variables|LoveLetter|SetCardManager _returnvalue)
      (Utilities|FlowControl|Sequence
        (:then_0
          (Class|UGCardManager|CreateGroup (Variables|LoveLetter|GetCardManager) 0 "Deck" "CGP_Secret" (Utilities|Array|Get(acopy) (Class|UGGame|GetBoundActorsbyTag "LLDeck")))
          (Class|UGCardManager|CreateGroup (Variables|LoveLetter|GetCardManager) 0 "RB" "CGP_Secret"))
        (:then_1
          (for _array_element (Variables|Default|GetPlayers)
            (bind _asllps (Utilities|Casting|CastToLLPS _array_element))
            (Class|UGCardManager|CreateGroup (Variables|LoveLetter|GetCardManager) _asllps "Table" "CGP_Public" (Default|GetBoundActorbyTag _asllps "LLTable"))
            (Class|UGCardManager|CreateGroup (Variables|LoveLetter|GetCardManager) _asllps "Hand" "CGP_Private" (Default|GetBoundActorbyTag _asllps "LLHand"))))))
    (:then_1
      (for _array_element_2 (Variables|LoveLetter|GetPack)
        (bind _returnvalue_2 (Game|SpawnActorfromClass _array_element_2 (Math|Transform|MakeTransform "0, 0, 0") "Undefined" 0 0))
        (Class|UGCardManager|RegisterCard (Variables|LoveLetter|GetCardManager) _returnvalue_2 0 "Deck")))))

(event Custom|Draw
  (params (Player :type LLPS%20Object%20Reference))
  ;[1 1 1] Draw
  (if (Variables|/Script/UnrealGames.UGPS|GetbIsInGame Player)
    (Class|UGGame|Log (Utilities|Text|FormatText "{Player} draws a card." (Utilities|Text|ToText(String) (Variables|/Script/Engine.PlayerState|GetPlayerName Player))))
    (bind _returnvalue (Class|UGCardManager|PopTop (Variables|LoveLetter|GetCardManager) "Deck" Player "Hand"))
    (if (not _returnvalue)
      (Variables|Default|SetbRoundOver true)
      (Class|UGGame|Log (Utilities|Text|FormatText "No they don't. Deck is empty."))
      (Class|UGGame|EndTurn))))

(event Custom|ExecuteCard
  (params (Player :type LLPS%20Object%20Reference) (Card :type LL%20Base%20Card%20Object%20Reference) (Target :type LLPS%20Object%20Reference) (Value :type Integer))
  (bind _group (Variables|/Script/UnrealGames.UGCard|GetGroup Card))
  ;[1 1 1] Execute a card
  ;;[1 1 1] Validation
  ;;;[1 1 1] Card Validation
  (if (Math|Boolean|ANDBoolean (Variables|/Script/UnrealGames.UGPS|GetbMyTurn Player) (== Player (Components|GetOwner _group)) (Utilities|Name|Equal(Name) (Variables|/Script/UnrealGames.UGCardGroup|GetCardGroupName _group) "Hand")) ; If it's his turn and he's activating his card
    (if (Variables|/Game/Games/LoveLetter/Blueprints/LLBaseCard.LLBaseCard_C|GetNeedsTarget Card)
      ;;;[1 1 1] Target Validation
      (Utilities|IsValid Target
        (:Is%20Valid
          (if (Variables|/Script/UnrealGames.UGPS|GetbIsInGame Target)
            (bind _allowed (Default|AllowedtoActivate Card :!label _label))
            (if _allowed
              (CallFunction|DiscardACard Card)
              (Default|Execute Card Player Target (Math|Integer|Clamp(Integer) Value 2 8))))))
      (else
        (goto _label)))))

(event Custom|Discard
  (params (Player :type LLPS%20Object%20Reference))
  (bind _cardmanager (Variables|LoveLetter|GetCardManager))
  (bind _returnvalue (Class|UGCardManager|GetGroup _cardmanager Player "Hand"))
  (bind _cards (Variables|/Script/UnrealGames.UGCardGroup|GetCards _returnvalue))
  ;[1 1 1] Discard
  (if (> (Utilities|Array|Length _cards) 0)
    (bind _asllbase_card (Utilities|Casting|CastToLLBaseCard (Utilities|Array|Get(acopy) _cards)))
    (CallFunction|DiscardACard _asllbase_card)
    (else
      (Development|PrintText (Utilities|Text|FormatText "{0} has nothing to discard." (Utilities|Text|ToText(String) (Variables|/Script/Engine.PlayerState|GetPlayerName Player))) false))))

(event Custom|Discard%20a%20Card
  (params (Card :type LL%20Base%20Card%20Object%20Reference))
  (bind _value (Variables|/Game/Games/LoveLetter/Blueprints/LLBaseCard.LLBaseCard_C|GetValue Card))
  (bind _cardname (Variables|/Script/UnrealGames.UGCard|GetCardName Card))
  ;[1 1 1] Discard
  (bind _asllps (Utilities|Casting|CastToLLPS (Components|GetOwner (Variables|/Script/UnrealGames.UGCard|GetGroup Card))))
  (Development|PrintText (Utilities|Text|FormatText "{0} discards {1}." (Utilities|Text|ToText(String) (Variables|/Script/Engine.PlayerState|GetPlayerName _asllps)) _cardname) false)
  (bind _returnvalue (Class|UGCardManager|PushTop (Variables|LoveLetter|GetCardManager) Card _asllps "Table"))
  (if _returnvalue
    (Class|UGGame|Log (Utilities|Text|FormatText "{Player} discards {Card}." (Utilities|Text|ToText(String) (Variables|/Script/Engine.PlayerState|GetPlayerName _asllps)) _cardname))
    (bind _output_get (Variables|/Game/Games/LoveLetter/Blueprints/LLPS.LLPS_C|SetRoundScore _asllps (+ _value (stale _output_get))))
    (bind _output_get_2 (Variables|/Game/Games/LoveLetter/Blueprints/LLPS.LLPS_C|SetCardsDiscarded _asllps (+ (stale _output_get_2) 1)))
    (if (== _value 8)
      (Class|UGGame|LoseRound _asllps))))

(fn ConstructionScript)

(fn GetWinners
  (bind _winners (LocalVariables|GetWinners))
  (bind _winners_2 (LocalVariables|GetWinners))
  (bind _item (Utilities|Array|Get(acopy) _winners))
  (bind _roundscore (Variables|/Game/Games/LoveLetter/Blueprints/LLPS.LLPS_C|GetRoundScore _item))
  (bind _returnvalue (|CallParentFunction))
  (for _array_element _returnvalue
    (bind _asllps (Utilities|Casting|CastToLLPS _array_element))
    (if (== (Utilities|Array|Length (Variables|/Script/UnrealGames.UGCardGroup|GetCards (Class|UGCardManager|GetGroup (Variables|LoveLetter|GetCardManager) _array_element "Hand"))) 0)
      (Class|UGCardManager|PopTop (Variables|LoveLetter|GetCardManager) "RB" _asllps "Hand"))
    (if (== (Utilities|Array|Length (LocalVariables|GetWinners)) 0)
      (Utilities|Array|Add (LocalVariables|GetWinners) _asllps)
      (else
        (bind _asllbase_card (Utilities|Casting|CastToLLBaseCard (Utilities|Array|Get(acopy) (Variables|/Script/UnrealGames.UGCardGroup|GetCards (Class|UGCardManager|GetGroup (Variables|LoveLetter|GetCardManager) _asllps "Hand")))))
        (if (> (Variables|/Game/Games/LoveLetter/Blueprints/LLBaseCard.LLBaseCard_C|GetValue _asllbase_card) (LocalVariables|GetWinnersHand))
          (LocalVariables|SetWinnersHand (Variables|/Game/Games/LoveLetter/Blueprints/LLBaseCard.LLBaseCard_C|GetValue _asllbase_card))
          (Utilities|Array|Clear _winners_2 :!label _label)
          (Utilities|Array|Add _winners_2 _asllps :!label _label_2)
          (elif (== (Variables|/Game/Games/LoveLetter/Blueprints/LLBaseCard.LLBaseCard_C|GetValue _asllbase_card) (LocalVariables|GetWinnersHand))
            (if (> (Variables|/Game/Games/LoveLetter/Blueprints/LLPS.LLPS_C|GetRoundScore _asllps) _roundscore)
              (goto _label)
              (elif (== (Variables|/Game/Games/LoveLetter/Blueprints/LLPS.LLPS_C|GetRoundScore _asllps) _roundscore)
                (goto _label_2))))))))
  ;[1 1 1] Winner starts next round
  (Variables|Default|SetCurPlayerIndex (Utilities|Array|FindItem (Variables|Default|GetPlayers) (Utilities|Array|Get(acopy) (LocalVariables|GetWinners))))
  (return (LocalVariables|GetWinners)))