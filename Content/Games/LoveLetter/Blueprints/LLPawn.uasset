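; Player pawn for the Love Letter card game that displays a two-card hand on skeletal mesh sockets and supports FOV zoom.
; BeginPlay spawns hidden physical cards with particles and links non-local pawns to their widget.
; UGCardGroupViz updates refresh the cards, setting each face through a dynamic material's Card Index.
; Tick bobs cards with layered sine waves eased between timer-randomized frequencies, and shows MagicHorn while the visualizer is active.
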(event UpdateVisualizer(UGCardGroupViz)
  (bind _ugcardgroupviz (Variables|Default|GetUGCardGroupViz))
  (bind _ugcardgroupviz_2 (Variables|Default|GetUGCardGroupViz))
  (bind _returnvalue (Class|UGCardGroupVizComponent|GetGroup _ugcardgroupviz))
  (bind _info (Variables|/Script/UnrealGames.UGCardGroupVizComponent|GetInfo _ugcardgroupviz_2))
  (Networking|SwitchHasAuthority
    (:Authority
      _)
    (:Remote
      (Development|PrintString "Update Hand" false true "(R=0.000000,G=0.660000,B=1.000000,A=1.000000)" 2.0)))
  (if (Math|Conversions|ToBoolean(Integer) (Utilities|Array|Length (Variables|Cards|GetHandRenderedCards)))
    (Utilities|FlowControl|Sequence
      (:then_0
        (for _array_element (Variables|Cards|GetHandRenderedCards)
          (Rendering|SetActorHiddenInGame _array_element true)))
      (:then_1
        (Utilities|IsValid _info
          (:Is%20Valid
            (for _index (range 0 (- (Variables|/Script/UnrealGames.UGCardGroupInfo|GetCardCount _info) 1))
              (bind _returnvalue_2 (Rendering|Material|CreateDynamicMaterialInstance "/Game/Games/LoveLetter/Materials/M_LLCard_Back.M_LLCard_Back" :!class /Script/Engine.KismetMaterialLibrary))
              (Utilities|IsValid _returnvalue
                (:Is%20Valid
                  (bind _asllbase_card (Utilities|Casting|CastToLLBaseCard (Utilities|Array|Get(acopy) (Variables|/Script/UnrealGames.UGCardGroup|GetCards _returnvalue) _index))
                    (:then
                      (Rendering|Material|SetScalarParameterValue _returnvalue_2 "Card Index" (Math|Conversions|ToFloat(Integer) (- (Variables|/Game/Games/LoveLetter/Blueprints/LLBaseCard.LLBaseCard_C|GetValue _asllbase_card) 1)) :!class /Script/Engine.MaterialInstanceDynamic))
                    (:CastFailed
                      _)))
                (:Is%20Not%20Valid
                  _))
              (Variables|/Game/Generic/UGPhysicalCard.UGPhysicalCard_C|SetCard (Utilities|Array|Get(acopy) (Variables|Cards|GetHandRenderedCards) _index) _asllbase_card)
              (Variables|/Game/Generic/UGPhysicalCard.UGPhysicalCard_C|SetFrontMaterial (Utilities|Array|Get(acopy) (Variables|Cards|GetHandRenderedCards) _index) _returnvalue_2)
              (Default|Update (Utilities|Array|Get(acopy) (Variables|Cards|GetHandRenderedCards) _index))
              (Rendering|SetActorHiddenInGame (Utilities|Array|Get(acopy) (Variables|Cards|GetHandRenderedCards) _index) false))))))
    (else
      (Development|PrintString "Update Hand Failed" true true "(R=0.000000,G=0.660000,B=1.000000,A=1.000000)" 2.0))))

(event EventBeginPlay
  (bind _self self)
  (bind _ugcardgroupviz (Variables|Default|GetUGCardGroupViz))
  (bind _ugcardgroupviz_2 (Variables|Default|GetUGCardGroupViz))
  (bind _returnvalue (Class|UGCardGroupVizComponent|GetGroup _ugcardgroupviz))
  (bind _info (Variables|/Script/UnrealGames.UGCardGroupVizComponent|GetInfo _ugcardgroupviz_2))
  ;[1 1 1] Begin Play
  (|CallParentFunction)
  (for _index (range 0 1)
    (bind _returnvalue_2 (Game|SpawnActorfromClass "/Game/Generic/UGPhysicalCard.UGPhysicalCard_C" (Math|Transform|MakeTransform "0, 0, 0" "0, 0, 0" "1000.000000,1,1") "AlwaysSpawn" _self "/Game/Games/LoveLetter/Materials/M_LLCard_Back.M_LLCard_Back" "/Game/Games/LoveLetter/Materials/M_LLCard_Back.M_LLCard_Back" 0 false (Variables|Default|GetUGCardGroupViz) _self))
    (Class|Actor|AttachRootComponentto _returnvalue_2 (Variables|Default|GetSkeletalMesh) (Utilities|Array|Get(acopy) (Variables|Cards|GetHandSpawnPoints) _index) "SnapToTargetIncludingScale" true)
    (Effects|SpawnEmitterAttached "/Game/Graphics/Particles/MagicCard2.MagicCard2" (Variables|/Game/Generic/UGPhysicalCard.UGPhysicalCard_C|GetMesh _returnvalue_2) "None")
    (Rendering|SetActorHiddenInGame _returnvalue_2 true)
    (Utilities|Array|Add (Variables|Cards|GetHandRenderedCards) _returnvalue_2))
  (Utilities|FlowControl|Sequence
    (:then_0
      (if (not (Pawn|IsLocallyControlled))
        (bind _asllpawn_widget (Utilities|Casting|CastToLLPawnWidget (UserInterface|GetUserWidgetObject (Variables|Default|GetWidget))))
        (Variables|/Game/Games/LoveLetter/Blueprints/LLPawnWidget.LLPawnWidget_C|SetPawn _asllpawn_widget self)))
    (:then_1
      (CallFunction|InitAnimtaion))
    (:then_2
      (Networking|SwitchHasAuthority
        (:Authority
          _)
        (:Remote
          (Development|PrintString "Update Hand" false true "(R=0.000000,G=0.660000,B=1.000000,A=1.000000)" 2.0)))
      (if (Math|Conversions|ToBoolean(Integer) (Utilities|Array|Length (Variables|Cards|GetHandRenderedCards)))
        (Utilities|FlowControl|Sequence
          (:then_0
            (for _array_element (Variables|Cards|GetHandRenderedCards)
              (Rendering|SetActorHiddenInGame _array_element true)))
          (:then_1
            (Utilities|IsValid _info
              (:Is%20Valid
                (for _index_2 (range 0 (- (Variables|/Script/UnrealGames.UGCardGroupInfo|GetCardCount _info) 1))
                  (bind _returnvalue_3 (Rendering|Material|CreateDynamicMaterialInstance "/Game/Games/LoveLetter/Materials/M_LLCard_Back.M_LLCard_Back" :!class /Script/Engine.KismetMaterialLibrary))
                  (Utilities|IsValid _returnvalue
                    (:Is%20Valid
                      (bind _asllbase_card (Utilities|Casting|CastToLLBaseCard (Utilities|Array|Get(acopy) (Variables|/Script/UnrealGames.UGCardGroup|GetCards _returnvalue) _index_2))
                        (:then
                          (Rendering|Material|SetScalarParameterValue _returnvalue_3 "Card Index" (Math|Conversions|ToFloat(Integer) (- (Variables|/Game/Games/LoveLetter/Blueprints/LLBaseCard.LLBaseCard_C|GetValue _asllbase_card) 1)) :!class /Script/Engine.MaterialInstanceDynamic))
                        (:CastFailed
                          _)))
                    (:Is%20Not%20Valid
                      _))
                  (Variables|/Game/Generic/UGPhysicalCard.UGPhysicalCard_C|SetCard (Utilities|Array|Get(acopy) (Variables|Cards|GetHandRenderedCards) _index_2) _asllbase_card)
                  (Variables|/Game/Generic/UGPhysicalCard.UGPhysicalCard_C|SetFrontMaterial (Utilities|Array|Get(acopy) (Variables|Cards|GetHandRenderedCards) _index_2) _returnvalue_3)
                  (Default|Update (Utilities|Array|Get(acopy) (Variables|Cards|GetHandRenderedCards) _index_2))
                  (Rendering|SetActorHiddenInGame (Utilities|Array|Get(acopy) (Variables|Cards|GetHandRenderedCards) _index_2) false))))))
        (else
          (Development|PrintString "Update Hand Failed" true true "(R=0.000000,G=0.660000,B=1.000000,A=1.000000)" 2.0))))))

(event EventTick
  (params (DeltaSeconds :type Float%20%28single-precision%29))
  (|CallParentFunction DeltaSeconds)
  (CallFunction|UpdateAnimation))

(event EventOnReset
  (bind _handrenderedcards (Variables|Cards|GetHandRenderedCards))
  (|CallParentFunction)
  (for _array_element _handrenderedcards
    (Actor|DestroyActor _array_element))
  (Utilities|Array|Clear _handrenderedcards))

(event Input|ActionEvents|InputActionZoomIn
  (params (Key :type Key%20Structure :default "AnyKey"))
  (bind _camera (Variables|Default|GetCamera))
  (:Pressed
    (Variables|Default|SetTempFloat -1.0)
    (Variables|/Script/Engine.CameraComponent|SetFieldOfView _camera (Math|Float|Clamp(Float) (+ (Variables|/Script/Engine.CameraComponent|GetFieldOfView _camera) (* (Variables|Default|GetTempFloat) (Variables|Default|GetFOVStep))) 25.0 9e+01))))

(event Input|ActionEvents|InputActionZoomOut
  (params (Key :type Key%20Structure :default "AnyKey"))
  (bind _camera (Variables|Default|GetCamera))
  (:Pressed
    (Variables|Default|SetTempFloat 1.0)
    (Variables|/Script/Engine.CameraComponent|SetFieldOfView _camera (Math|Float|Clamp(Float) (+ (Variables|/Script/Engine.CameraComponent|GetFieldOfView _camera) (* (Variables|Default|GetTempFloat) (Variables|Default|GetFOVStep))) 25.0 9e+01))))

(event Custom|RandomizeAnimation
  (Variables|Cards|SetAnimOldX (Variables|Cards|GetAnimRandomX))
  (Variables|Cards|SetAnimRandomX (Math|Random|RandomFloat))
  (Variables|Cards|SetAnimOldY (Variables|Cards|GetAnimRandomY))
  (Variables|Cards|SetAnimRandomY (Math|Random|RandomFloat)))

(event Custom|Init%20Animtaion
  (Variables|Cards|SetAnimShift (Math|Float|MultiplybyPi (Math|Random|RandomFloat)))
  (bind _returnvalue (Utilities|Time|SetTimerbyEvent (delegate Custom|RandomizeAnimation) 1.0 true))
  (Variables|Cards|SetAnimTimer _returnvalue))

(event Custom|Update%20Animation
  (bind _animtimer (Variables|Cards|GetAnimTimer))
  (bind _returnvalue (Class|KismetSystemLibrary|GetTimerElapsedTimeHandle _animtimer))
  (for (_array_element _array_index) (Variables|Cards|GetHandRenderedCards)
    (Transformation|SetRelativeLocation (Variables|/Game/Generic/UGPhysicalCard.UGPhysicalCard_C|GetMesh _array_element) (Math|Vector|MakeVector (+ (* (Math|Trig|Cos(Radians) (+ (Utilities|Time|GetGameTimeinSeconds) (Variables|Cards|GetAnimShift) (Math|Conversions|ToFloat(Integer) _array_index))) 1.0) (* (Math|Trig|Cos(Radians) (* (+ (Utilities|Time|GetGameTimeinSeconds) (Variables|Cards|GetAnimShift) (Math|Conversions|ToFloat(Integer) _array_index)) (+ (Class|KismetMathLibrary|FInterpEaseinOut (Variables|Cards|GetAnimOldX) (Variables|Cards|GetAnimRandomX) _returnvalue 2.0) 1.0) 0.4)) 0.25)) 0.0 (+ (* (Math|Trig|Sin(Radians) (+ (Utilities|Time|GetGameTimeinSeconds) (Variables|Cards|GetAnimShift) (Math|Conversions|ToFloat(Integer) _array_index))) 2.5) (* (Math|Trig|Sin(Radians) (* (+ (Utilities|Time|GetGameTimeinSeconds) (Variables|Cards|GetAnimShift) (Math|Conversions|ToFloat(Integer) _array_index)) (+ (Class|KismetMathLibrary|FInterpEaseinOut (Variables|Cards|GetAnimOldY) (Variables|Cards|GetAnimRandomY) _returnvalue 2.0) 1.0) 0.4)) 0.5))) false false))
  (Rendering|SetVisibility (Variables|Default|GetMagicHorn) (Components|Activation|IsActive (Variables|Default|GetUGCardGroupViz)) false))

(fn ConstructionScript
  (bind _handspawnpoints (Variables|Cards|GetHandSpawnPoints))
  (|CallParentFunction)
  (Utilities|Array|Add _handspawnpoints "Socket_Hand0")
  (Utilities|Array|Add _handspawnpoints "Socket_Hand1"))