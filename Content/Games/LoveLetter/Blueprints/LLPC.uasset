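; Player controller for the Love Letter card game, bridging card choices between the HUD widget and game mode.
; Card prompts store the active card and open value or target pickers, auto-selecting when fewer than two targets qualify.
; Chosen passes the selection back to that card, while ServerActivate forwards plays to Game_LoveLetter for execution.
; Learn reveals another player's card, and Cancel or Pause hides the widget.
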(event EventBeginPlay
  (|CallParentFunction)
  (CallFunction|DeactivateMouseCursor))

(event Custom|Choose%20Value
  (params (Card :type LL%20Base%20Card%20Object%20Reference))
  (Development|PrintText "Choose value" false)
  (Variables|Default|SetActiveCard Card)
  (bind _asllhud (Utilities|Casting|CastToLLHUD (HUD|GetHUD)))
  (Default|ChooseValue (Variables|/Game/Games/LoveLetter/Blueprints/LLHUD.LLHUD_C|GetLLWidget _asllhud))
  (CallFunction|ActivateMouseCursor (Variables|/Game/Games/LoveLetter/Blueprints/LLHUD.LLHUD_C|GetLLWidget _asllhud)))

(event Custom|Choose%20Player
  (params (Can%20Choose%20Self :type Boolean) (Card :type LL%20Base%20Card%20Object%20Reference))
  (bind _targetlist (Variables|Default|GetTargetList))
  (Development|PrintText "Choose target" false)
  (Variables|Default|SetActiveCard Card)
  (Utilities|Array|Clear (Variables|Default|GetTargetList))
  (if Can%20Choose%20Self
    (bind _asllps (Utilities|Casting|CastToLLPS (Variables|Default|GetPlayerState)))
    (Utilities|Array|Add (Variables|Default|GetTargetList) _asllps))
  (bind _outactors (Actor|GetAllActorsOfClass "/Game/Games/LoveLetter/Blueprints/LLPS.LLPS_C"))
  (for _array_element _outactors
    (if (and (Variables|/Script/UnrealGames.UGPS|GetbIsInGame _array_element) (!= _array_element (Variables|Default|GetPlayerState)))
      (Utilities|Array|Add (Variables|Default|GetTargetList) _array_element)))
  (Utilities|FlowControl|Sequence
    (:then_0
      (for _array_element_2 _targetlist
        (Development|PrintString (Variables|/Script/Engine.PlayerState|GetPlayerName _array_element_2) false true "(R=1.000000,G=0.000000,B=0.117710,A=1.000000)" 1e+01)))
    (:then_1
      (if (>= (Utilities|Array|Length _targetlist) 2)
        (bind _asllhud (Utilities|Casting|CastToLLHUD (HUD|GetHUD)))
        (Default|ChooseTarget (Variables|/Game/Games/LoveLetter/Blueprints/LLHUD.LLHUD_C|GetLLWidget _asllhud) (Variables|Default|GetTargetList))
        (CallFunction|ActivateMouseCursor (Variables|/Game/Games/LoveLetter/Blueprints/LLHUD.LLHUD_C|GetLLWidget _asllhud))
        (else
          (CallFunction|Chosen (Utilities|Array|Get(acopy) _targetlist)))))))

(event Custom|ServerActivate
  (params (Card :type LL%20Base%20Card%20Object%20Reference) (Target :type LLPS%20Object%20Reference) (Value :type Integer))
  (bind _asllps (Utilities|Casting|CastToLLPS (Variables|Default|GetPlayerState))
    (:then
      (bind _asgame_love_letter (Utilities|Casting|CastToGame_LoveLetter (Game|GetGameMode))
        (:then
          (Default|ExecuteCard _asgame_love_letter _asllps Card Target Value))
        (:CastFailed
          (Development|PrintText "Love Letter Card: Wrong game!" false :!label _label))))
    (:CastFailed
      (goto _label))))

(event Custom|Learn
  (params (Other%20Player :type Player%20State%20Object%20Reference) (Value :type Integer))
  (bind _asllhud (Utilities|Casting|CastToLLHUD (HUD|GetHUD)))
  (Default|ShowCard (Variables|/Game/Games/LoveLetter/Blueprints/LLHUD.LLHUD_C|GetLLWidget _asllhud) (Variables|/Script/Engine.PlayerState|GetPlayerName Other%20Player) Value)
  (CallFunction|ActivateMouseCursor (Variables|/Game/Games/LoveLetter/Blueprints/LLHUD.LLHUD_C|GetLLWidget _asllhud)))

(event Custom|Chosen
  (params (Player :type Player%20State%20Object%20Reference) (Value :type Integer))
  (bind _activecard (Variables|Default|GetActiveCard))
  (CallFunction|DeactivateMouseCursor)
  (Development|PrintText "Chosen" false)
  (bind _asllps (Utilities|Casting|CastToLLPS Player)
    (:then
      (Default|Chosen _activecard _asllps Value))
    (:CastFailed
      (Default|Chosen _activecard 0 Value))))

(event Custom|Turn)

(event Input|ActionEvents|InputActionCancel
  (params (Key :type Key%20Structure :default "AnyKey"))
  (:Released
    (CallFunction|DeactivateMouseCursor)
    (bind _asllhud (Utilities|Casting|CastToLLHUD (HUD|GetHUD)))
    (Default|HideAll (Variables|/Game/Games/LoveLetter/Blueprints/LLHUD.LLHUD_C|GetLLWidget _asllhud))))

(event Input|ActionEvents|InputActionPause
  (params (Key :type Key%20Structure :default "AnyKey"))
  (:Pressed
    (bind _asllhud (Utilities|Casting|CastToLLHUD (HUD|GetHUD)))
    (Default|HideAll (Variables|/Game/Games/LoveLetter/Blueprints/LLHUD.LLHUD_C|GetLLWidget _asllhud))))

(fn ConstructionScript
  (|CallParentFunction))