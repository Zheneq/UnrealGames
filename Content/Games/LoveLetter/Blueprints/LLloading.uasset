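; Love Letter loading actor, apparently an animated card shown while the game loads.
; The construction script stores a dynamic instance of the card back material as FrontMaterial, with a random card index.
; BeginPlay applies a slight random pitch and yaw, then starts a timeline that sets absolute world location from its scaled track.
; The timeline reverses each time it finishes, producing an endless ping-pong motion.
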(event EventBeginPlay
  (|CallParentFunction)
  (Transformation|SetActorRotation (Math|Rotator|MakeRotator 0.0 (Math|Random|RandomFloatinRange -1e+01 1e+01) (Math|Random|RandomFloatinRange -1e+01 1e+01)))
  (bind (_direction _newtrack_0) (Timeline|Animation Play)
    (:Update
      (Transformation|SetActorLocation (* _newtrack_0 1e+02) false false))
    (:Finished
      (switch Utilities|FlowControl|Switch|SwitchonETimelineDirection _direction
        (:Forward
          (Timeline|Animation ReverseFromEnd))
        (:Backward
          (Timeline|Animation PlayFromStart))))))

(fn ConstructionScript
  (|CallParentFunction)
  (bind _returnvalue (Rendering|Material|CreateDynamicMaterialInstance "/Game/Games/LoveLetter/Materials/M_LLCard_Back.M_LLCard_Back" :!class /Script/Engine.KismetMaterialLibrary))
  (Variables|Default|SetFrontMaterial _returnvalue)
  (Rendering|Material|SetScalarParameterValue _returnvalue "Card Index" (Math|Conversions|ToFloat(Integer) (Math|Random|RandomIntegerinRange 0 8)) :!class /Script/Engine.MaterialInstanceDynamic))