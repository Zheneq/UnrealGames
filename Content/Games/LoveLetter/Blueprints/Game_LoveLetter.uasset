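; Game mode for the Love Letter card game, running player joins, turns, eliminations and round ends.
; It spawns a UGCardManager holding a secret deck, a set-aside pile and per-player hand and table groups.
; Card plays are validated, discarded to the table for score, then executed, with discarding an 8 eliminating its owner.
; Rounds end on an empty deck or through elimination, comparing hand values, then discard totals.
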(event Custom|Draw
  (params (Player :type LLPS%20Object%20Reference))
  ;[1 1 1] Draw
  (bind _returnvalue (Class|UGCardManager|PopTop (Variables|Default|GetCardManager) "Deck" Player "Hand"))
  (if (not _returnvalue)
    (CallFunction|EndTurn Player)
    (CallFunction|EndRound)))

(event Custom|End%20Round
  ;[1 1 1] Round End
  (bind _players_count (CallFunction|GetinGamePlayersCount))
  (switch int _players_count
    (:Default
      (bind _winners (CallFunction|FindWinners))
      (Variables|Default|SetCurPlayerIndex (Utilities|Array|FindItem (Variables|Default|GetPlayers) (Utilities|Array|Get(acopy) _winners)))
      (CallFunction|RoundOver _winners))
    (:0
      (Development|PrintText "It's weird. Nobody won." false)
      (CallFunction|RoundOver (Utilities|Array|MakeArray 0)))
    (:1
      (CallFunction|RoundOver (Utilities|Array|MakeArray (Utilities|Array|Get(acopy) (Variables|Default|GetPlayers) (Variables|Default|GetCurPlayerIndex)))))))

(event EventPreInitRound
  (bind _cardmanager (Variables|Default|GetCardManager))
  ;[1 1 1] Reset Round
  (Class|UGCardManager|Restart _cardmanager)
  (Class|UGCardManager|Shuffle _cardmanager 0 "Deck")
  (Class|UGCardManager|PopTop _cardmanager "Deck" 0 "RB"))

(event EventGameTurn
  (params (Player :type UGPS%20BP%20Object%20Reference))
  ;[1 1 1] Game Turn
  (bind _asllps (Utilities|Casting|CastToLLPS Player))
  (Variables|/Game/Games/LoveLetter/Blueprints/LLPS.LLPS_C|SetProtected _asllps false)
  (bind _returnvalue (Class|UGCardManager|PopTop (Variables|Default|GetCardManager) "Deck" _asllps "Hand"))
  (if _returnvalue
    (bind _asllpc (Utilities|Casting|CastToLLPC (Components|GetOwner Player)))
    (Default|Turn _asllpc)
    (else
      (CallFunction|EndRound))))

(event EventLose
  (params (Pl :type UGPS%20Object%20Reference))
  (|CallParentFunction Pl)
  (bind _asllps (Utilities|Casting|CastToLLPS Pl))
  (CallFunction|Discard _asllps))

(event EventPostLogin
  (params (NewPlayer :type Player%20Controller%20Object%20Reference))
  (if (not (Variables|Default|GetIsInGame))
    (bind _asllps (Utilities|Casting|CastToLLPS (Variables|/Script/Engine.Controller|GetPlayerState NewPlayer)))
    (Utilities|Array|Add (Variables|Default|GetPlayers) _asllps)
    (bind _asuggi_bp (Utilities|Casting|CastToUGGI_BP (Game|GetGameInstance)))
    (if (>= (Variables|Default|GetNumPlayers) (Variables|/Game/Generic/UGGI_BP.UGGI_BP_C|GetTemp_PlayersCount _asuggi_bp))
      (Utilities|FlowControl|Delay 2.0)
      (CallFunction|StartGame))))

(event EventOnLogout
  (params (ExitingController :type Controller%20Object%20Reference))
  (bind _asllps (Utilities|Casting|CastToLLPS (Variables|/Script/Engine.Controller|GetPlayerState ExitingController)))
  (CallFunction|KickPlayer _asllps))

(event EventPreInitGame
  (Utilities|FlowControl|Sequence
    (:then_0
      ;[1 1 1] Init CardManager
      (bind _returnvalue (Game|SpawnActorfromClass "/Script/UnrealGames.UGCardManager" (Math|Transform|MakeTransform "0, 0, 0") "AlwaysSpawn" self 0))
      (Variables|Default|SetCardManager _returnvalue)
      (Utilities|FlowControl|Sequence
        (:then_0
          (Class|UGCardManager|CreateGroup (Variables|Default|GetCardManager) 0 "Deck" "CGP_Secret" (Utilities|Array|Get(acopy) (CallFunction|GetBoundActorsbyTag "LLDeck")))
          (Class|UGCardManager|CreateGroup (Variables|Default|GetCardManager) 0 "RB" "CGP_Secret"))
        (:then_1
          (for _array_element (Variables|Default|GetPlayers)
            (bind _asllps (Utilities|Casting|CastToLLPS _array_element))
            (Class|UGCardManager|CreateGroup (Variables|Default|GetCardManager) _asllps "Table" "CGP_Public" (Variables|/Game/Games/LoveLetter/Blueprints/LLPS.LLPS_C|GetTableRenderer _asllps))
            (Class|UGCardManager|CreateGroup (Variables|Default|GetCardManager) _asllps "Hand" "CGP_Private" (Variables|/Game/Games/LoveLetter/Blueprints/LLPS.LLPS_C|GetHandRenderer _asllps))))))
    (:then_1
      (for _array_element_2 (Variables|Default|GetPack)
        (bind _returnvalue_2 (Game|SpawnActorfromClass _array_element_2 (Math|Transform|MakeTransform "0, 0, 0") "Undefined" 0 0))
        (Class|UGCardManager|RegisterCard (Variables|Default|GetCardManager) _returnvalue_2 0 "Deck")))))

(event EventInitPlayer
  (params (Index :type Integer) (Player :type UGPS%20BP%20Object%20Reference))
  ;[1 1 1] Init Player
  (bind _asllps (Utilities|Casting|CastToLLPS Player))
  (Variables|/Game/Games/LoveLetter/Blueprints/LLPS.LLPS_C|SetRoundScore _asllps 0)
  (Variables|/Game/Games/LoveLetter/Blueprints/LLPS.LLPS_C|SetCardsDiscarded _asllps 0)
  (CallFunction|Draw _asllps))

(event EventTick
  (params (DeltaSeconds :type Float%20%28single-precision%29))
  (bind _asuggi_bp (Utilities|Casting|CastToUGGI_BP (Game|GetGameInstance)))
  (if (Variables|/Game/Generic/UGGI_BP.UGGI_BP_C|GetDebugMode _asuggi_bp)
    (bind _returnvalue (Class|GameMode|GetNumPlayers))
    (Development|PrintString (Utilities|String|Append "Active players: " (Utilities|String|ToString(Integer) _returnvalue) ", spectators: " (Utilities|String|ToString(Integer) (Variables|Default|GetNumSpectators)) ",  travelling players: " (Utilities|String|ToString(Integer) (Variables|Default|GetNumTravellingPlayers))) true true "(R=0.000000,G=0.660000,B=1.000000,A=1.000000)" 0.01)))

(event Custom|ExecuteCard
  (params (Player :type LLPS%20Object%20Reference) (Card :type LL%20Base%20Card%20Object%20Reference) (Target :type LLPS%20Object%20Reference) (Value :type Integer))
  (bind _group (Variables|/Script/UnrealGames.UGCard|GetGroup Card))
  ;[1 1 1] Validation
  ;;[1 1 1] Card Validation
  (if (Math|Boolean|ANDBoolean (Variables|/Script/UnrealGames.UGPS|GetbMyTurn Player) (== Player (Components|GetOwner _group)) (Utilities|Name|Equal(Name) (Variables|/Script/UnrealGames.UGCardGroup|GetCardGroupName _group) "Hand")) ; If it's his turn and he's activating his card
    (if (Variables|/Game/Games/LoveLetter/Blueprints/LLBaseCard.LLBaseCard_C|GetNeedsTarget Card)
      ;;[1 1 1] Target Validation
      (Utilities|IsValid Target
        (:Is%20Valid
          (if (Variables|/Script/UnrealGames.UGPS|GetbIsInGame Target)
            (bind _allowed (Default|AllowedtoActivate Card :!label _label))
            (if _allowed
              (CallFunction|DiscardACard Card)
              (Default|Execute Card Player Target (Math|Integer|Clamp(Integer) Value 2 8))))))
      (else
        (goto _label)))))

(event Custom|Discard
  (params (Player :type LLPS%20Object%20Reference))
  (bind _cardmanager (Variables|Default|GetCardManager))
  (bind _returnvalue (Class|UGCardManager|GetGroup _cardmanager Player "Hand"))
  (bind _cards (Variables|/Script/UnrealGames.UGCardGroup|GetCards _returnvalue))
  ;[1 1 1] Discard
  (if (> (Utilities|Array|Length _cards) 0)
    (bind _asllbase_card (Utilities|Casting|CastToLLBaseCard (Utilities|Array|Get(acopy) _cards)))
    (CallFunction|DiscardACard _asllbase_card)
    (else
      (Development|PrintText (Utilities|Text|FormatText "{0} has nothing to discard." (Utilities|Text|ToText(String) (Variables|/Script/Engine.PlayerState|GetPlayerName Player))) false))))

(event Custom|Discard%20a%20Card
  (params (Card :type LL%20Base%20Card%20Object%20Reference))
  (bind _value (Variables|/Game/Games/LoveLetter/Blueprints/LLBaseCard.LLBaseCard_C|GetValue Card))
  ;[1 1 1] Discard
  (bind _asllps (Utilities|Casting|CastToLLPS (Components|GetOwner (Variables|/Script/UnrealGames.UGCard|GetGroup Card))))
  (Development|PrintText (Utilities|Text|FormatText "{0} discards a card ({1})." (Utilities|Text|ToText(String) (Variables|/Script/Engine.PlayerState|GetPlayerName _asllps)) (Variables|/Script/UnrealGames.UGCard|GetCardName Card)) false)
  (bind _returnvalue (Class|UGCardManager|PushTop (Variables|Default|GetCardManager) Card _asllps "Table"))
  (if _returnvalue
    (bind _output_get (Variables|/Game/Games/LoveLetter/Blueprints/LLPS.LLPS_C|SetRoundScore _asllps (+ _value (stale _output_get))))
    (bind _output_get_2 (Variables|/Game/Games/LoveLetter/Blueprints/LLPS.LLPS_C|SetCardsDiscarded _asllps (+ (stale _output_get_2) 1)))
    (if (== _value 8)
      (CallFunction|Lose _asllps))))

(fn ConstructionScript
  (|CallParentFunction))

(fn FindWinners
  (bind _winnersstates (LocalVariables|GetWinnersStates))
  (bind _winnersstates_2 (LocalVariables|GetWinnersStates))
  (bind _item (Utilities|Array|Get(acopy) _winnersstates))
  (bind _roundscore (Variables|/Game/Games/LoveLetter/Blueprints/LLPS.LLPS_C|GetRoundScore _item))
  (bind _array_element (Utilities|Array|ForEachLoopwithBreak (Variables|Default|GetPlayers) :!label _label)
    (:LoopBody
      (if (Variables|/Script/UnrealGames.UGPS|GetbIsInGame _array_element)
        (bind _asllps (Utilities|Casting|CastToLLPS _array_element))
        (Utilities|Array|Add (LocalVariables|GetWinnersStates) _asllps)
        (Variables|/Script/UnrealGames.UGPS|SetbIsInGame _asllps false)
        (goto _label Break)))
    (:Completed
      (for _array_element_2 (Variables|Default|GetPlayers)
        (bind _asllps_2 (Utilities|Casting|CastToLLPS _array_element_2))
        (if (Variables|/Script/UnrealGames.UGPS|GetbIsInGame _array_element_2)
          (bind _asllbase_card (Utilities|Casting|CastToLLBaseCard (Utilities|Array|Get(acopy) (Variables|/Script/UnrealGames.UGCardGroup|GetCards (Class|UGCardManager|GetGroup (Variables|Default|GetCardManager) _asllps_2 "Hand")))))
          (if (> (Variables|/Game/Games/LoveLetter/Blueprints/LLBaseCard.LLBaseCard_C|GetValue _asllbase_card) (LocalVariables|GetWinnerHand))
            (LocalVariables|SetWinnerHand (Variables|/Game/Games/LoveLetter/Blueprints/LLBaseCard.LLBaseCard_C|GetValue _asllbase_card))
            (Utilities|Array|Clear _winnersstates_2 :!label _label_2)
            (Utilities|Array|Add _winnersstates_2 _asllps_2 :!label _label_3)
            (elif (== (Variables|/Game/Games/LoveLetter/Blueprints/LLBaseCard.LLBaseCard_C|GetValue _asllbase_card) (LocalVariables|GetWinnerHand))
              (if (> (Variables|/Game/Games/LoveLetter/Blueprints/LLPS.LLPS_C|GetRoundScore _asllps_2) _roundscore)
                (goto _label_2)
                (elif (== (Variables|/Game/Games/LoveLetter/Blueprints/LLPS.LLPS_C|GetRoundScore _asllps_2) _roundscore)
                  (goto _label_3)))))))
      (return (LocalVariables|GetWinnersStates)))))