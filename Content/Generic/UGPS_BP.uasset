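; UGPS_BP is a player state Blueprint that tracks whether a player is in the game and whether it is their turn.
; Both flags have RepNotify handlers, which are empty here, as are the Init event and construction script.
; GetController returns the owner cast to a Controller.
; GetAvatar lazily fetches and caches the Steam avatar while the avatar is still the default white grid texture.
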(event Custom|Init)

(fn ConstructionScript)

(fn OnRepMyTurn)

(fn OnRepIsinGame)

(fn GetController
  (bind _ascontroller (Utilities|Casting|CastToController (Components|GetOwner))
    (:then
      (return _ascontroller))
    (:CastFailed
      (return 0))))

(fn GetAvatar
  (if (== (Variables|UnrealGames|GetAvatar) "/Engine/EngineMaterials/DefaultWhiteGrid.DefaultWhiteGrid")
    (bind _returnvalue (Class|UGPS|GetSteamAvatar))
    (bind _output_get (Variables|UnrealGames|SetAvatar _returnvalue)))
  (return _output_get))