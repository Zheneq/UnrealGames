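; Game mode Blueprint that spawns each player's pawn at a claimed UGPlayerStart and starts the game once everybody connects.
; Tick polls HasEverybodyConnected, then calls StartGame once after a short delay.
; Default pawn spawning reuses the player's assigned start or claims the first free one, then spawns, possesses and initializes the player.
; The player-count capacity check is unfinished and currently bypassed.
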(event EventTick
  (params (DeltaSeconds :type Float%20%28single-precision%29))
  (Utilities|FlowControl|Gate false :!label _label
    (:Exit
      (if (Class|UGGM|HasEverybodyConnected)
        (Utilities|FlowControl|DoOnce false
          (:Completed
            (Utilities|FlowControl|Delay 2.0)
            (Class|UGGame|StartGame (Class|UGFunctionLibrary|GetGame))
            (goto _label Close)))))))

(fn ConstructionScript)

(fn SpawnDefaultPawnfor
  (params (NewPlayer :type Controller%20Object%20Reference) (StartSpot :type Actor%20Object%20Reference))
  (bind _asugps_bp (Utilities|Casting|CastToUGPS_BP (Variables|/Script/Engine.Controller|GetPlayerState NewPlayer))
    (:then
      (bind _pawn (CallFunction|SpawnAPawnforPlayer _asugps_bp))
      (return _pawn))
    (:CastFailed
      (return 0))))

(fn SpawnAPawnforPlayer
  (params (Player :type UGPS%20BP%20Object%20Reference))
  (bind _returnvalue (Components|GetOwner Player))
  ;[1 0 0] TODO: Check if we have enough space
  (bind _returnvalue_2 (Class|GameMode|GetNumPlayers))
  (if true
    (Utilities|IsValid (Variables|/Game/Generic/UGPS_BP.UGPS_BP_C|GetPlayerStart Player)
      (:Is%20Valid
        (if (== (Variables|/Game/Generic/UGPlayerStart.UGPlayerStart_C|GetPlayer (Variables|/Game/Generic/UGPS_BP.UGPS_BP_C|GetPlayerStart Player)) Player) ; If the new player know where to spawn, just spawn him. If not, try to find a place
          _
          (else
            (bind _outactors (Actor|GetAllActorsOfClass "/Game/Generic/UGPlayerStart.UGPlayerStart_C" :!label _label))
            (bind _array_element (Utilities|Array|ForEachLoopwithBreak _outactors :!label _label_2)
              (:LoopBody
                (Utilities|IsValid (Variables|/Game/Generic/UGPlayerStart.UGPlayerStart_C|GetPlayer _array_element)
                  (:Is%20Not%20Valid
                    (bind _output_get (Variables|/Game/Generic/UGPlayerStart.UGPlayerStart_C|SetPlayer _array_element Player))
                    (Variables|/Game/Generic/UGPS_BP.UGPS_BP_C|SetPlayerStart _output_get _array_element)
                    (goto _label_2 Break))))
              (:Completed
                (Utilities|IsValid (Variables|/Game/Generic/UGPS_BP.UGPS_BP_C|GetPlayerStart Player)
                  (:Is%20Valid
                    _)
                  (:Is%20Not%20Valid
                    (return 0))))))))
      (:Is%20Not%20Valid
        (goto _label)))
    (bind _pawn_class (CallFunction|UGGetDefaultPawnClass Player))
    (bind _returnvalue_3 (Game|SpawnActorfromClass _pawn_class (Transformation|GetActorTransform (Variables|/Game/Generic/UGPS_BP.UGPS_BP_C|GetPlayerStart Player)) "AdjustIfPossibleButAlwaysSpawn" _returnvalue 0))
    (Utilities|Array|Add (Variables|/Game/Generic/UGPlayerStart.UGPlayerStart_C|GetBoundActors (Variables|/Game/Generic/UGPS_BP.UGPS_BP_C|GetPlayerStart Player)) _returnvalue_3)
    (bind _ascontroller (Utilities|Casting|CastToController _returnvalue)
      (:then
        (Pawn|Possess _ascontroller _returnvalue_3)
        (Default|Init Player)
        (return _returnvalue_3))
      (:CastFailed
        (return 0)))
    (else
      (return 0))))

(fn UGGetDefaultPawnClass
  (params (Player :type UGPS%20BP%20Object%20Reference))
  (bind _asugpawn (Utilities|Casting|CastToUGPawnClass (Variables|Default|GetDefaultPawnClass))
    (:then
      (return _asugpawn))
    (:CastFailed
      (return "/Game/Generic/UGPawn.UGPawn_C"))))