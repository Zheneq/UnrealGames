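; Game instance Blueprint (UGGI) that manages online session flow and a stacked menu system.
; Hosts listen servers (game mode option ignored due to an engine bug) and joins sessions; session failures and travel or network errors fall back to MainMenu, destroying the session.
; Menus are cached per class and stacked: OpenMenu prunes invalid entries and swaps the visible widget, while MenuReturn restores the previous one or game input, notifying widgets through MenuInterface.
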(event Custom|Host%20Game
  (params (Level%20Name :type Name) (Game%20Mode :type Name) (LAN :type Boolean) (Max%20Players :type Integer))
  (bind _returnvalue (Game|GetPlayerController 0))
  (if (and (Utilities|Name|NotEqual(Name) Level%20Name "None") (> Max%20Players 0))
    (|Session _returnvalue Max%20Players LAN
      (:OnSuccess
        (if (Utilities|Name|Equal(Name) Game%20Mode "None")
          (Variables|Default|SetLevelURL "listen")
          (else
            (Variables|Default|SetLevelURL (Utilities|String|Append "listen&game=" (Utilities|String|ToString(Name) Game%20Mode)))))
        (Game|OpenLevel(byName) Level%20Name true "listen") ; GameMode is ignored now because ofa bug in the engine
      )
      (:OnFailure
        (|DestroySession _returnvalue
          (:then
            (Development|PrintText "Failed to create online session." true true "(R=0.000000,G=0.660000,B=1.000000,A=1.000000)" 2e+01)
            (CallFunction|GotoMainMenu)))))))

(event Custom|Go%20To%20Main%20Menu
  (bind _returnvalue (Game|GetGameMode))
  (|DestroySession (Game|GetPlayerController 0)
    (:then
      (Utilities|IsValid _returnvalue
        (:Is%20Valid
          (Variables|/Script/Engine.GameMode|SetbUseSeamlessTravel _returnvalue false))
        (:Is%20Not%20Valid
          _))
      (Game|OpenLevel(byName) "MainMenu"))))

(event Custom|Join%20Game
  (params (Server :type Blueprint%20Session%20Result%20Structure))
  (bind _returnvalue (Game|GetPlayerController 0))
  (|JoinSession _returnvalue Server
    (:OnFailure
      (|DestroySession _returnvalue
        (:then
          (Development|PrintText "Failed to join online session." true true "(R=0.000000,G=0.660000,B=1.000000,A=1.000000)" 2e+01)
          (CallFunction|GotoMainMenu))))))

(event EventHandleTravelError
  (params (FailureType :type ETravelFailure%20Enum :default "NoLevel"))
  ;[1 1 1] Errors
  (Development|PrintString (Utilities|String|EnumtoString FailureType) true true "(R=0.683427,G=0.001751,B=1.000000,A=1.000000)" 15.0)
  (CallFunction|GotoMainMenu))

(event EventHandleNetworkError
  (params (FailureType :type ENetworkFailure%20Enum :default "NetDriverAlreadyExists") (bIsServer :type Boolean))
  ;[1 1 1] Errors
  (Development|PrintString (Utilities|String|EnumtoString FailureType) true true "(R=1.000000,G=0.000000,B=0.000000,A=1.000000)" 15.0)
  (CallFunction|GotoMainMenu))

(fn GetMenu
  (params (Menu :type User%20Widget%20Class%20Reference))
  (bind _cachedmenus (Variables|UnrealGames|Menu|GetCachedMenus))
  (bind _cachedmenusrefs (Variables|UnrealGames|Menu|GetCachedMenusRefs))
  (bind _returnvalue (Utilities|Array|FindItem _cachedmenus Menu))
  (bind _item (Utilities|Array|Get(acopy) _cachedmenusrefs _returnvalue))
  (if (== _returnvalue -1)
    (bind _returnvalue_2 (UserInterface|CreateWidget Menu (Game|GetPlayerController 0) :!label _label))
    (bind _output_get (LocalVariables|SetResult _returnvalue_2))
    (Utilities|Array|Add (Variables|UnrealGames|Menu|GetCachedMenusRefs) _output_get)
    (Utilities|Array|Add (Variables|UnrealGames|Menu|GetCachedMenus) Menu)
    (else
      (Utilities|IsValid _item
        (:Is%20Valid
          (LocalVariables|SetResult _item))
        (:Is%20Not%20Valid
          (Utilities|Array|RemoveIndex (Variables|UnrealGames|Menu|GetCachedMenusRefs) _returnvalue)
          (Utilities|Array|RemoveIndex (Variables|UnrealGames|Menu|GetCachedMenus) _returnvalue)
          (goto _label)))))
  (return (LocalVariables|GetResult)))

(fn MenuReturn
  (bind _returnvalue (Game|GetPlayerController 0))
  (bind _menustack (Variables|UnrealGames|Menu|GetMenuStack))
  (bind _menustack_2 (Variables|UnrealGames|Menu|GetMenuStack))
  (bind _returnvalue_2 (Utilities|Array|LastIndex _menustack))
  (bind _returnvalue_3 (Utilities|Array|LastIndex _menustack_2))
  (bind _item (Utilities|Array|Get(acopy) _menustack _returnvalue_2))
  (if (>= _returnvalue_3 1)
    (bind _output_get (LocalVariables|SetLastMenu (Utilities|Array|Get(acopy) _menustack_2 _returnvalue_3)))
    (Widget|RemovefromParent _output_get)
    (Utilities|Array|RemoveIndex _menustack _returnvalue_3)
    (Utilities|IsValid _item
      (:Is%20Valid
        (UserInterface|Viewport|AddtoViewport _item 0)
        (Input|SetInputModeUIOnly (Game|GetPlayerController 0) _item (Variables|UnrealGames|Menu|GetLockMouseToViewport))
        (if (Utilities|DoesObjectImplementInterface _item "/Game/Generic/MenuInterface.MenuInterface_C")
          (Class|MenuInterface|Returnedfrom(Message) _item (LocalVariables|GetLastMenu))
          (Development|PrintString "MenuReturn: Returned." false)))
      (:Is%20Not%20Valid
        (bind _asugpc_bp (Utilities|Casting|CastToUGPC_BP _returnvalue)
          (:then
            (Default|DeactivateMouseCursor _asugpc_bp))
          (:CastFailed
            (Input|SetInputModeGameOnly _returnvalue)))
        (Development|PrintString "MenuReturn: Closed all menus." false)))
    (else
      (Development|PrintString "MenuReturn: No menu opened!"))))

(fn OpenMenu
  (params (Menu :type User%20Widget%20Class%20Reference))
  (bind _menustack (Variables|UnrealGames|Menu|GetMenuStack))
  (bind _returnvalue (Utilities|Array|LastIndex _menustack))
  (bind _item (Utilities|Array|Get(acopy) _menustack _returnvalue))
  (bind _widget (UnrealGames|Menu|GetMenu Menu))
  (CallFunction|FixUpMenuStack)
  (Utilities|IsValid _item
    (:Is%20Valid
      (Widget|RemovefromParent _item))
    (:Is%20Not%20Valid
      _))
  (UserInterface|Viewport|AddtoViewport _widget 0)
  (Input|SetInputModeUIOnly (Game|GetPlayerController 0) _widget (Variables|UnrealGames|Menu|GetLockMouseToViewport))
  (if (Utilities|DoesObjectImplementInterface _widget "/Game/Generic/MenuInterface.MenuInterface_C")
    (Class|MenuInterface|Openedfrom(Message) _widget _item))
  (if (!= _widget _item)
    (Utilities|Array|Add (Variables|UnrealGames|Menu|GetMenuStack) _widget))
  (return _widget))

(fn FixUpMenuStack
  (LocalVariables|Seti 1)
  (if (<= (LocalVariables|Geti) (Utilities|Array|LastIndex (Variables|UnrealGames|Menu|GetMenuStack))) :!label _label
    (if (not (Utilities|IsValid (Utilities|Array|Get(acopy) (Variables|UnrealGames|Menu|GetMenuStack) (LocalVariables|Geti))))
      (Utilities|Array|RemoveIndex (Variables|UnrealGames|Menu|GetMenuStack) (stale _output_get))
      (goto _label)
      (else
        (bind _output_get (LocalVariables|Seti (+ (stale _output_get) 1)))
        (goto _label)))))