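; UGGS_BP is a game state Blueprint that relays replicated game information to the local player's controller and HUD.
; On BeginPlay it sets input focus to the game viewport.
; When Game replicates, it tells UGPC_BP on player controller 0 to update lobby game parameters.
; When GameDisplayName replicates, it has the UGHUD's widget refresh the displayed game name.
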(event EventOnRepGame
  (bind _asugpc_bp (Utilities|Casting|CastToUGPC_BP (Game|GetPlayerController 0)))
  (Default|LobbyUpdateGameParams _asugpc_bp))

(event EventBeginPlay
  (Class|WidgetBlueprintLibrary|SetFocustoGameViewport))

(event EventTick
  (params (DeltaSeconds :type Float%20%28single-precision%29)))

(fn ConstructionScript)

(fn OnRepGameDisplayName
  (bind _asughud (Utilities|Casting|CastToUGHUD (HUD|GetHUD (Game|GetPlayerController 0))))
  (Default|UpdateGameName (Variables|/Game/Generic/UGHUD.UGHUD_C|GetWidget _asughud)))