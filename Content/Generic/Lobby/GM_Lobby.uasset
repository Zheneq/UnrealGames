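; Lobby game mode that sets up joining players and relays lobby changes to every connected UGPC player controller.
; On login it shows the new player's lobby widget, then sends them the level and game names read from player controller 0's lobby widget.
; Settings updates and start-game notices are broadcast by looping over all UGPC actors and calling the matching event on each.
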(event Custom|NotifyStartGame
  (bind _outactors (Actor|GetAllActorsOfClass "/Game/Generic/UGPC.UGPC_C"))
  (for _array_element _outactors
    (Default|LobbyStartGameNotify _array_element)))

(event Custom|LobbyUpdateSettings
  (params (Level :type Name) (Game :type Name))
  (bind _outactors (Actor|GetAllActorsOfClass "/Game/Generic/UGPC.UGPC_C"))
  (for _array_element _outactors
    (Default|LobbyUpdateSettings _array_element Level Game)))

(event EventPostLogin
  (params (NewPlayer :type Player%20Controller%20Object%20Reference))
  (bind _asugpc (Utilities|Casting|CastToUGPC NewPlayer))
  (Default|ShowLobbyWidget _asugpc)
  (bind _asugpc_2 (Utilities|Casting|CastToUGPC (Game|GetPlayerController 0)))
  (Default|LobbyUpdateSettings _asugpc (Variables|/Game/Generic/Lobby/W_Lobby.W_Lobby_C|GetLevelName (Variables|/Game/Generic/UGPC.UGPC_C|GetLobbyWidget _asugpc_2)) (Variables|/Game/Generic/Lobby/W_Lobby.W_Lobby_C|GetGameName (Variables|/Game/Generic/UGPC.UGPC_C|GetLobbyWidget _asugpc_2))))

(fn ConstructionScript)