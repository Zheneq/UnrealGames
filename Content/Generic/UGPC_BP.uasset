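; Player controller that handles first-person interaction, cursor/input-mode switching, and lobby UI with chat.
; Click release and mouse-idle hover share a line or sphere trace from the pawn camera to UGInteractInterface actors, sending click messages or spawning hover popups that look movement dismisses.
; Chat messages fan out to every UGPC_BP's chat widget.
; Lobby events open the menu, forward level/game settings, and show a loading widget until seamless travel ends.
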(event Custom|Activate%20Mouse%20Cursor
  (params (In%20Widget%20To%20Focus :type Widget%20Object%20Reference))
  ;[1 1 1] Show/Hide Cursor
  ;;[1 0.06737 0.1343] This part is ignored now
  (bind _output_get (Variables|Default|SetCursorBlockCount (Math|Integer|Clamp(Integer) (- (stale _output_get) 1) 0 1000)))
  (if (== _output_get 0)
    _
    (else
      _))
  (Input|SetIgnoreLookInput true)
  (Variables|Default|SetbShowMouseCursor true)
  (Input|SetInputModeGameandUI self In%20Widget%20To%20Focus true true)
  (Development|PrintText "Mouse cursor activated." false))

(event Custom|Deactivate%20Mouse%20Cursor
  ;[1 1 1] Show/Hide Cursor
  ;;[1 0.06737 0.1343] This part is ignored now
  (bind _output_get (Variables|Default|SetCursorBlockCount (+ (stale _output_get) 1)))
  (Input|SetIgnoreLookInput false)
  (Variables|Default|SetbShowMouseCursor false)
  (Class|WidgetBlueprintLibrary|SetFocustoGameViewport)
  (Input|SetInputModeGameOnly self)
  (Development|PrintText "Mouse cursor deactivated." false))

(event EventTick
  (params (DeltaSeconds :type Float%20%28single-precision%29))
  ;[1 1 1] Tooltips
  (|CallParentFunction DeltaSeconds)
  (if (Pawn|IsLocalPlayerController)
    (if (and (< (Variables|UnrealGamesUI|GetHoverDelay) (- (Utilities|Time|GetGameTimeinSeconds) (Variables|UnrealGamesUI|GetLastMoveTimestamp))) (not (Utilities|IsValid (Variables|UnrealGamesUI|GetHoverWidgetObject))))
      (Utilities|FlowControl|Sequence
        (:then_0
          (bind _asuggi_bp (Utilities|Casting|CastToUGGI_BP (Game|GetGameInstance)))
          (Development|PrintString "Hover" (Variables|/Game/Generic/UGGI_BP.UGGI_BP_C|GetDebugMode _asuggi_bp))
          (if (or (not (Variables|Default|GetbShowMouseCursor)) (not (Variables|UnrealGamesUI|GetIgnore%20Clicks%20When%20in%20UI)))
            (bind _hit_actor (CallFunction|Trace))
            (Utilities|IsValid _hit_actor
              (:Is%20Valid
                (if (Utilities|DoesObjectImplementInterface _hit_actor "/Game/Generic/UGInteractInterface.UGInteractInterface_C")
                  (bind _returnvalue (Game|SpawnActorfromClass "/Game/Generic/UGPopUpWidget.UGPopUpWidget_C" (Math|Transform|MakeTransform "0, 0, 0") "AlwaysSpawn" 0 _hit_actor "/Game/Generic/UGWidget_Hover.UGWidget_Hover_C"))
                  (Variables|UnrealGamesUI|SetHoverWidgetObject _returnvalue))))))
        (:then_1
          (Variables|UnrealGamesUI|SetLastMoveTimestamp (Class|UGFunctionLibrary|Infinity)))))))

(event Input|ActionEvents|InputActionClick
  (params (Key :type Key%20Structure :default "AnyKey"))
  ;[1 1 1] Click
  (:Released
    (Class|WidgetBlueprintLibrary|SetFocustoGameViewport)
    (if (or (not (Variables|Default|GetbShowMouseCursor)) (not (Variables|UnrealGamesUI|GetIgnore%20Clicks%20When%20in%20UI)))
      (bind _hit_actor (CallFunction|Trace))
      (if (and (Utilities|IsValid _hit_actor) (Utilities|DoesObjectImplementInterface _hit_actor "/Game/Generic/UGInteractInterface.UGInteractInterface_C"))
        (Class|UGInteractInterface|Clicked(Message) _hit_actor Key)
        (Development|PrintString (Utilities|String|Append "Clicked " (Utilities|GetDisplayName _hit_actor)) false)))))

(event Input|AxisEvents|InputAxisTurn
  (params (AxisValue :type Float%20%28single-precision%29))
  ;[1 1 1] Tooltips
  (if (!= AxisValue 0.0)
    (Variables|UnrealGamesUI|SetLastMoveTimestamp (Utilities|Time|GetGameTimeinSeconds))
    (Utilities|IsValid (Variables|UnrealGamesUI|GetHoverWidgetObject)
      (:Is%20Valid
        (Default|Hide (Variables|/Game/Generic/UGPopUpWidget.UGPopUpWidget_C|GetWidget (Variables|UnrealGamesUI|GetHoverWidgetObject)))
        (Variables|UnrealGamesUI|SetHoverWidgetObject 0)))))

(event Input|AxisEvents|InputAxisLookUp
  (params (AxisValue :type Float%20%28single-precision%29))
  ;[1 1 1] Tooltips
  (if (!= AxisValue 0.0)
    (Variables|UnrealGamesUI|SetLastMoveTimestamp (Utilities|Time|GetGameTimeinSeconds))
    (Utilities|IsValid (Variables|UnrealGamesUI|GetHoverWidgetObject)
      (:Is%20Valid
        (Default|Hide (Variables|/Game/Generic/UGPopUpWidget.UGPopUpWidget_C|GetWidget (Variables|UnrealGamesUI|GetHoverWidgetObject)))
        (Variables|UnrealGamesUI|SetHoverWidgetObject 0)))))

(event Custom|LobbyStartGameNotify
  (bind _asuggi_bp (Utilities|Casting|CastToUGGI_BP (Game|GetGameInstance)))
  (Default|MenuReturn _asuggi_bp)
  (CallFunction|ShowLoadingWidget))

(event Custom|ShowLobbyWidget
  (bind _asuggi_bp (Utilities|Casting|CastToUGGI_BP (Game|GetGameInstance)))
  (bind _menureference (Default|OpenMenu _asuggi_bp "/Game/Generic/Lobby/W_Lobby.W_Lobby_C"))
  (bind _asw_lobby (Utilities|Casting|CastToW_Lobby _menureference))
  (Variables|Default|SetLobbyWidget _asw_lobby))

(event Custom|ShowLoadingWidget
  (bind _returnvalue (UserInterface|CreateWidget "/Game/Generic/MainMenu/W_Loading.W_Loading_C" self))
  (bind _output_get (Variables|Default|SetLoadingWidget _returnvalue))
  (UserInterface|Viewport|AddtoViewport _output_get 0))

(event Custom|LobbyUpdateSettings
  (params (Level :type Name) (Game :type Name))
  (bind _lobbywidget (Variables|Default|GetLobbyWidget))
  (Utilities|IsValid _lobbywidget
    (:Is%20Valid
      (Default|ReplicateSettings _lobbywidget Level Game))))

(event Custom|ChatSendMessage
  (params (Message :type String))
  (bind _outactors (Actor|GetAllActorsOfClass "UGPC_BP_C"))
  (for _array_element _outactors
    (bind _asugps_bp (Utilities|Casting|CastToUGPS_BP (Variables|Default|GetPlayerState)))
    (CallFunction|ChatRecieveMessage _array_element _asugps_bp Message)))

(event Custom|ChatRecieveMessage
  (params (Sender :type UGPS%20BP%20Object%20Reference) (Message :type String))
  (bind _chatwidget (Variables|Default|GetChatWidget))
  (Utilities|IsValid _chatwidget
    (:Is%20Valid
      (Default|RecieveMessage _chatwidget Sender Message))))

(event EventOnEndSeamlessTravel
  (Widget|RemovefromParent (Variables|Default|GetLoadingWidget)))

(fn ConstructionScript)

(fn Trace
  (bind _returnvalue (Pawn|GetControlledPawn))
  (Utilities|IsValid _returnvalue
    (:Is%20Valid
      (bind _desiredview (Class|CameraComponent|GetCameraView (Utilities|Array|Get(acopy) (Actor|GetComponentsByClass _returnvalue "/Script/Engine.CameraComponent")) 0.0))
      (bind _asuggi_bp (Utilities|Casting|CastToUGGI_BP (Game|GetGameInstance))
        (:then
          (bind (_out_hit _return_value) (CallFunction|TraceSub (.Location (Utilities|Struct|BreakMinimalViewInfo _desiredview)) (+ (.Location (Utilities|Struct|BreakMinimalViewInfo _desiredview)) (* (Math|Rotator|GetRotationXVector (.Rotation (Utilities|Struct|BreakMinimalViewInfo _desiredview))) (Variables|UnrealGamesUI|GetTrace%20Distance))) (Utilities|Array|MakeArray (Pawn|GetControlledPawn)) (select (Variables|/Game/Generic/UGGI_BP.UGGI_BP_C|GetDebugMode _asuggi_bp) "ForDuration" "None")))
          (if _return_value
            (Development|PrintString (Utilities|String|Append "Trace: hit " (Utilities|GetDisplayName (.HitActor (Collision|BreakHitResult _out_hit)))) (Variables|/Game/Generic/UGGI_BP.UGGI_BP_C|GetDebugMode _asuggi_bp))
            (return (.HitActor (Collision|BreakHitResult _out_hit)))
            (else
              (Development|PrintString "Trace: hit nothing" (Variables|/Game/Generic/UGGI_BP.UGGI_BP_C|GetDebugMode _asuggi_bp))
              (return 0))))
        (:CastFailed
          (return 0))))
    (:Is%20Not%20Valid
      (Development|PrintString "Trace failed: No pawn")
      (return 0))))

(fn TraceSub
  (params (Start :type Vector) (End :type Vector) (ActorsToIgnore :type Array%20of%20Actor%20Object%20References) (DrawDebugType :type EDrawDebugTrace%20Enum))
  (if (Variables|UnrealGamesUI|GetUseSphereTrace)
    (bind (_outhit _returnvalue) (Class|KismetSystemLibrary|SphereTraceSingleNEW Start End 1.0 "TraceTypeQuery1" false ActorsToIgnore DrawDebugType true))
    (return _outhit _returnvalue)
    (else
      (bind (_outhit_2 _returnvalue_2) (Collision|LineTraceByChannel Start End "TraceTypeQuery1" false ActorsToIgnore DrawDebugType))
      (return _outhit_2 _returnvalue_2))))